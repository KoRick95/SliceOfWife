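; BP_Soul is an AI actor that rotates every tick to face the player's camera and offers a "Hit" HUD prompt.
; Player overlap with its Box calls IsFocused, whose timeline updates the button prompts on the PlayerHUD of the BP_Reception found at BeginPlay.
; End overlap also calls IsFocused, so IsUnfocused, which stops the timeline and collapses the prompt, is never called here.
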(event `self.ReceiveBeginPlay`
  (bind _returnvalue (`GameplayStatics.GetActorOfClass` "/Game/Blueprints/InteractableEnvironment/BP_Reception.BP_Reception_C"))
  (set `self.BP_Reception` _returnvalue))

(event `self.Box.OnComponentBeginOverlap`
  (params (OverlappedComponent :type "PrimitiveComponent Object Reference") (OtherActor :type "Actor Object Reference") (OtherComp :type "PrimitiveComponent Object Reference") (OtherBodyIndex :type Integer) (bFromSweep :type Boolean) (SweepResult :type "HitResult Structure (by ref)"))
  (bind _playerchar (message `/Game/Blueprints/Interfaces/INT_PlayerCharacter.PlayerCharRef` OtherActor))
  (if (== _playerchar OtherActor)
    (`self.IsFocused`)))

(event `self.Box.OnComponentEndOverlap`
  (params (OverlappedComponent :type "PrimitiveComponent Object Reference") (OtherActor :type "Actor Object Reference") (OtherComp :type "PrimitiveComponent Object Reference") (OtherBodyIndex :type Integer))
  (bind _playerchar (message `/Game/Blueprints/Interfaces/INT_PlayerCharacter.PlayerCharRef` OtherActor))
  (if (== _playerchar OtherActor)
    (`self.IsFocused`)))

(event `IsFocused`
  (bind _playerhud (`/Game/Blueprints/InteractableEnvironment/BP_Reception.PlayerHUD` (`self.BP_Reception`)))
  (`Timeline|IsFocusedTimeline`
    (:`Update`
      (`TextBlock.SetText` (`/Game/Blueprints/UI/W_PlayerHUD.Button2Text` _playerhud) "Hit")
      (`Widget.SetVisibility` (`/Game/Blueprints/UI/W_PlayerHUD.Button2HBox` _playerhud) "Visible")
      (`Widget.SetVisibility` (`/Game/Blueprints/UI/W_PlayerHUD.Button1HBox` _playerhud) "Collapsed"))))

(event `IsUnfocused`
  (`TimelineComponent.Stop` (`self.IsFocusedTimeline`))
  (`Widget.SetVisibility` (`/Game/Blueprints/UI/W_PlayerHUD.Button2HBox` (`/Game/Blueprints/InteractableEnvironment/BP_Reception.PlayerHUD` (`self.BP_Reception`))) "Collapsed"))

(event `self.ReceiveTick`
  (params (DeltaSeconds :type "Float (single-precision)"))
  (`/Engine/EditorBlueprintResources/StandardMacros.IsValid` self
    (:`Is Valid`
      (`self.RotateTowardsPlayer`))))

(fn `RotateTowardsPlayer`
  (bind _playerchar (message `/Game/Blueprints/Interfaces/INT_PlayerCharacter.PlayerCharRef` (`GameplayStatics.GetPlayerCharacter` 0)))
  (`SceneComponent.K2_SetWorldRotation` (`self.DefaultSceneRoot`) (`KismetMathLibrary.FindLookAtRotation` (`SceneComponent.K2_GetComponentLocation` (`self.DefaultSceneRoot`)) (`SceneComponent.K2_GetComponentLocation` (`/Game/Blueprints/BP_MainCharacter.Camera` _playerchar))) false false))

(fn `UserConstructionScript`)