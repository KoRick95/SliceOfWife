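; AI character that travels along a referenced spline path, with random pauses along the way.
; When active at BeginPlay, it runs a timeline scaled to a set duration from a start offset, mapping alpha to spline distance for location and rotation.
; A random delay triggered from the timeline update leads to a coin-flip chance to stop for a few seconds before playback resumes.
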(event `self.ReceiveBeginPlay`
  (if (`self.Active`)
    (`self.StartMovement`)))

(event `StartMovement`
  (bind _movementtimeline (`self.MovementTimeline`))
  (bind _movementtimeline_2 (`self.MovementTimeline`))
  (bind _spline (`/Game/Blueprints/AI/BP_Path.Spline` (`self.PathRef`)))
  (bind _returnvalue (`KismetMathLibrary.Lerp` 0.0 (`SplineComponent.GetSplineLength` _spline) (`self.MovementAlpha`)))
  (`TimelineComponent.SetPlayRate` _movementtimeline_2 (/ 1.0 (`self.TimelineDuration`)))
  (`TimelineComponent.SetNewTime` _movementtimeline_2 (`self.StartOffset`))
  (bind (_direction _alpha) (`Timeline|MovementTimeline` :!via `PlayFromStart`)
    (:`Update`
      (set `self.MovementAlpha` _alpha)
      (`self.K2_SetActorLocationAndRotation` (`SplineComponent.GetLocationAtDistanceAlongSpline` _spline _returnvalue "World") (`SplineComponent.GetRotationAtDistanceAlongSpline` _spline _returnvalue "World"))
      (`KismetSystemLibrary.Delay` (`KismetMathLibrary.RandomFloatInRange` 5.0 60.0))
      (if (`self.M_Percentage` 50.0)
        (`TimelineComponent.Stop` _movementtimeline)
        (`KismetSystemLibrary.Delay` (`KismetMathLibrary.RandomFloatInRange` 5.0 10.0)))
      (`TimelineComponent.Play` _movementtimeline))))

(fn `UserConstructionScript`)