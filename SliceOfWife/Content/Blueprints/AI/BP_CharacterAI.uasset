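; BP_CharacterAI is an AI character that wanders the nav mesh around its spawn point when FollowsNavMesh is enabled.
; BeginPlay stores the spawn location, sets walk speed through SetMovementState, then starts Roaming.
; Roaming moves to random navigable points within RoamRadius, pausing randomly before repeating; a failed move prints a message and stops the loop.
; SetMovementState maps Idle, Walk and Sprint to movement speed, though only Walk is used here.
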(event `self.ReceiveBeginPlay`
  (if (`self.FollowsNavMesh`)
    (set `self.SpawnLocation` (`self.K2_GetActorLocation`))
    (`self.SetMovementState` "NewEnumerator1")
    (`self.Roaming`)))

(event `Roaming`
  (if (not (`self.IsRoaming`))
    (`|AIMoveTo` self (`NavigationSystemV1.K2_GetRandomLocationInNavigableRadius` (`self.SpawnLocation`) (`self.RoamRadius`) null null) null 70.0 true
      (:`then`
        (set `self.IsRoaming` true))
      (:`OnSuccess`
        (`KismetSystemLibrary.Delay` (`KismetMathLibrary.RandomFloatInRange` 2.0 5.0))
        (set `self.IsRoaming` false)
        (`self.Roaming`))
      (:`OnFail`
        (`KismetSystemLibrary.PrintString` "MoveToFail")))))

(fn `SetMovementState`
  (params (MovementState :type "/Game/Blueprints/Enums/E_MovementState Enum" :default "NewEnumerator0"))
  (bind _walkspeed (`self.WalkSpeed`))
  (set `CharacterMovementComponent.MaxWalkSpeed` (select `/Game/Blueprints/Enums/E_MovementState` MovementState :`NewEnumerator1` _walkspeed :`NewEnumerator2` (* _walkspeed (`self.SprintSpeedMultiplier`))) (`self.CharacterMovement`)))

(fn `UserConstructionScript`)