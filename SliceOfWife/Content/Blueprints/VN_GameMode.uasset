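; Visual novel game mode that sets up scene captures and the menu and dialogue UI when play begins.
; BeginPlay indexes every VN_SceneCapture2D actor by BackgroundName into a map.
; It then checks the game instance's menu widget: in-game it makes that menu transparent and hit-test invisible, otherwise it starts music through a dialogue widget value message.
; The dialogue widget is added to the viewport collapsed.
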(event `self.ReceiveBeginPlay`
  (bind _asvn_game_instance (cast `/Game/Blueprints/VN_GameInstance` (`GameplayStatics.GetGameInstance`) :!pure true))
  (bind _gameinsmenuwidget (`/Game/Blueprints/VN_GameInstance.GameInsMenuWidget` _asvn_game_instance))
  (bind _gameinsdialoguewidget (`/Game/Blueprints/VN_GameInstance.GameInsDialogueWidget` _asvn_game_instance))
  (bind _canvaspanel_0 (`/Game/Blueprints/DialogueSystem/W_VNMenu.CanvasPanel_0` _gameinsmenuwidget))
  (`|ExecutionSequence`
    (:`then_0`
      (bind _outactors (`GameplayStatics.GetAllActorsOfClass` "/Game/Blueprints/DialogueSystem/VN_SceneCapture2D.VN_SceneCapture2D_C"))
      (for _array_element _outactors
        (`BlueprintMapLibrary.Map_Add` (`self.VNSceneCaptures`) (`/Game/Blueprints/DialogueSystem/VN_SceneCapture2D.BackgroundName` _array_element) _array_element)))
    (:`then_1`
      ;[1 1 1] Show Game/Menu Widget
      (if (`/Game/Blueprints/DialogueSystem/W_VNMenu.IsInGame` _gameinsmenuwidget)
        (`Widget.SetRenderOpacity` _canvaspanel_0 0.0)
        (`Widget.SetVisibility` _canvaspanel_0 "HitTestInvisible")
        (else
          ;;[1 1 1] On start game music
          (message `DlgDialogueParticipant.ModifyNameValue` _gameinsdialoguewidget "ChangeMusic" "Kevin_MacLeod_-_Monkeys_Spinning_Monkeys")))
      (`UserWidget.AddToViewport` _gameinsdialoguewidget 0)
      (`Widget.SetVisibility` (`/Game/Blueprints/DialogueSystem/W_VNDialogue.CanvasPanel_0` _gameinsdialoguewidget) "Collapsed"))))

(fn `UserConstructionScript`)