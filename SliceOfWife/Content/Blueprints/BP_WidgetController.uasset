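; BP_WidgetController is an actor that forwards the player's Interact input to the level's BP_Reception actor.
; On BeginPlay it caches the VN_GameInstance, finds BP_Reception with GetActorOfClass, enables input on player controller 0 and prints a debug string.
; Pressing the Interact action calls Interact on the cached reception reference.
; The cached game instance is not used elsewhere in the graph.
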(event `self.ReceiveBeginPlay`
  (set `self.VN_GameInstance` (cast `/Game/Blueprints/VN_GameInstance` (`GameplayStatics.GetGameInstance`) :!pure true))
  (bind _returnvalue (`GameplayStatics.GetActorOfClass` "/Game/Blueprints/InteractableEnvironment/BP_Reception.BP_Reception_C"))
  (set `self.BP_Reception` _returnvalue)
  (`self.EnableInput` (`GameplayStatics.GetPlayerController` 0) null)
  (`KismetSystemLibrary.PrintString` "WidgetController"))

(event `InputAction|Interact`
  (params (Key :type "Key Structure"))
  (:`Pressed`
    (`/Game/Blueprints/InteractableEnvironment/BP_Reception.Interact` (`self.BP_Reception`))))

(fn `UserConstructionScript`)