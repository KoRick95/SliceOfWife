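; Aquarium body storage Blueprint that registers the fish creature in its creature pool on BeginPlay, on top of the parent's setup.
; Overlapping the cage mesh focuses the storage when the actor is the player character and the reception's quest has been received.
; The player leaving the cage unfocuses it regardless of quest state.
; Player checks compare the actor with the result of a PlayerCharRefMessage call.
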(event `self.ReceiveBeginPlay`
  (`parent.ReceiveBeginPlay`)
  (`KismetArrayLibrary.Array_AddUnique` (`self.CreaturePool`) "/Game/Blueprints/BodyStorages/Creature_Fish.Creature_Fish_C"))

(event `self.SM_Cage.OnComponentBeginOverlap`
  (params (OverlappedComponent :type "PrimitiveComponent Object Reference") (OtherActor :type "Actor Object Reference") (OtherComp :type "PrimitiveComponent Object Reference") (OtherBodyIndex :type Integer) (bFromSweep :type Boolean) (SweepResult :type "HitResult Structure (by ref)"))
  (bind _playerchar (message `/Game/Blueprints/Interfaces/INT_PlayerCharacter.PlayerCharRef` OtherActor))
  (if (and (== _playerchar OtherActor) (`/Game/Blueprints/InteractableEnvironment/BP_Reception.QuestReceived` (`self.BPReception`)))
    (`self.IsFocused`)))

(event `self.SM_Cage.OnComponentEndOverlap`
  (params (OverlappedComponent :type "PrimitiveComponent Object Reference") (OtherActor :type "Actor Object Reference") (OtherComp :type "PrimitiveComponent Object Reference") (OtherBodyIndex :type Integer))
  (bind _playerchar (message `/Game/Blueprints/Interfaces/INT_PlayerCharacter.PlayerCharRef` OtherActor))
  (if (== _playerchar OtherActor)
    (`self.IsUnfocused`)))

(fn `UserConstructionScript`
  (`parent.UserConstructionScript`))