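; Fish tank body storage that adds the fish creature to its creature pool and animates two fish meshes swimming inside it.
; A rate-scaled timeline drives a shared alpha that places each fish along its own spline, with a yaw offset for facing.
; Player overlap on the static mesh toggles focus.
; The container indicator gets a fish icon and shows either the game instance's fish limit or unlimited uses.
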(event `self.ReceiveBeginPlay`
  (`parent.ReceiveBeginPlay`)
  (`KismetArrayLibrary.Array_AddUnique` (`self.CreaturePool`) "/Game/Blueprints/BodyStorages/Creature_Fish.Creature_Fish_C")
  (`self.StartMovement`))

(event `StartMovement`
  (`TimelineComponent.SetPlayRate` (`self.MovementTimeline`) (/ 1.0 (`self.TimelineDuration`)))
  (bind (_direction _alpha) (`Timeline|MovementTimeline`)
    (:`Update`
      (set `self.MovementAlpha` _alpha)
      (`self.CalculateAndSetSplinePlusMesh` (`self.Spline`) (`self.Fish`))
      (`self.CalculateAndSetSplinePlusMesh` (`self.Spline1`) (`self.Fish1`)))))

(event `self.StaticMesh.OnComponentBeginOverlap`
  (params (OverlappedComponent :type "PrimitiveComponent Object Reference") (OtherActor :type "Actor Object Reference") (OtherComp :type "PrimitiveComponent Object Reference") (OtherBodyIndex :type Integer) (bFromSweep :type Boolean) (SweepResult :type "HitResult Structure (by ref)"))
  (bind _playerchar (message `/Game/Blueprints/Interfaces/INT_PlayerCharacter.PlayerCharRef` OtherActor))
  (if (== _playerchar OtherActor)
    (`self.IsFocused`)))

(event `self.StaticMesh.OnComponentEndOverlap`
  (params (OverlappedComponent :type "PrimitiveComponent Object Reference") (OtherActor :type "Actor Object Reference") (OtherComp :type "PrimitiveComponent Object Reference") (OtherBodyIndex :type Integer))
  (bind _playerchar (message `/Game/Blueprints/Interfaces/INT_PlayerCharacter.PlayerCharRef` OtherActor))
  (if (== _playerchar OtherActor)
    (`self.IsUnfocused`)))

(event `self.SetVariables`
  (bind _vn_gameinstance (`self.VN_GameInstance`))
  (`Image.SetBrushFromTexture` (`/Game/Blueprints/UI/W_ContainerIndicator.Img_ContainerType` (`self.ContainerIndicator`)) "/Game/Assets/Sprites/UI_Art/portraits/fish.fish" false)
  (if (`self.IsLimited`)
    (set `/Game/Blueprints/VN_GameInstance.MaxFishLimit` (`/Game/Blueprints/VN_GameInstance.MaxFishLimit` _vn_gameinstance) _vn_gameinstance)
    (else
      (`TextBlock.SetText` (`/Game/Blueprints/UI/W_ContainerIndicator.RemainingText` (`self.ContainerIndicator`)) "Uses: ∞"))))

(event `self.GetRemainingText`
  (if (`self.IsLimited`)
    (`self.SetRemainingText` (`/Game/Blueprints/VN_GameInstance.MaxFishLimit` (`self.VN_GameInstance`)))))

(fn `CalculateAndSetSplinePlusMesh`
  (params (Spline :type "SplineComponent Object Reference") (Fish :type "SceneComponent Object Reference"))
  (bind _returnvalue (`KismetMathLibrary.Lerp` 0.0 (`SplineComponent.GetSplineLength` Spline) (`self.MovementAlpha`)))
  (bind (_returnvalue_roll _returnvalue_pitch _returnvalue_yaw) (`KismetMathLibrary.BreakRotator` (`SplineComponent.GetRotationAtDistanceAlongSpline` Spline _returnvalue "World")))
  (`SceneComponent.K2_SetWorldLocationAndRotation` Fish (`SplineComponent.GetLocationAtDistanceAlongSpline` Spline _returnvalue "World") (`KismetMathLibrary.MakeRotator` _returnvalue_roll _returnvalue_pitch (+ _returnvalue_yaw -90.0)) false false))

(fn `UserConstructionScript`
  (`parent.UserConstructionScript`))