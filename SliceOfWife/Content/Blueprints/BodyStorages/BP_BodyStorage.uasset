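; Base Blueprint for body storage containers, showing a usage counter and a "Collect" prompt, with setup and count refresh left to child classes.
; The counter widget turns toward the player camera each tick and shows only when the storage is active and the player can pick up.
; Once the reception quest is received, box overlap plays a timeline that refreshes the count and toggles BP_Reception's HUD prompt, hiding it while the player holds an object.
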(event `self.ReceiveTick`
  (params (DeltaSeconds :type "Float (single-precision)"))
  (`self.RotateToPlayer` (`self.RemainingCount`))
  (bind _playerchar (message `/Game/Blueprints/Interfaces/INT_PlayerCharacter.PlayerCharRef` (`GameplayStatics.GetPlayerCharacter` 0)))
  (`SceneComponent.SetVisibility` (`self.RemainingCount`) (and (`MainCharacter.CanPickUp` _playerchar) (`self.IsActive`)) false))

(event `self.ReceiveBeginPlay`
  (bind _isactive (`self.IsActive`))
  (`SceneComponent.SetVisibility` (`self.SpotLight`) _isactive false)
  (if (not _isactive)
    (`SceneComponent.SetVisibility` (`self.RemainingCount`) false false))
  (bind _returnvalue (`GameplayStatics.GetActorOfClass` "/Game/Blueprints/InteractableEnvironment/BP_Reception.BP_Reception_C"))
  (set `self.BPReception` _returnvalue)
  (set `self.VN_GameInstance` (cast `/Game/Blueprints/VN_GameInstance` (`GameplayStatics.GetGameInstance`) :!pure true))
  (set `self.ContainerIndicator` (cast `/Game/Blueprints/UI/W_ContainerIndicator` (`WidgetComponent.GetUserWidgetObject` (`self.RemainingCount`)) :!pure true))
  (`self.GetRemainingText`)
  (`self.SetVariables`))

(event `IsFocused`
  (bind _playerhud (`/Game/Blueprints/InteractableEnvironment/BP_Reception.PlayerHUD` (`self.BPReception`)))
  (bind _button1hbox (`/Game/Blueprints/UI/W_PlayerHUD.Button1HBox` _playerhud))
  (`Timeline|IsFocusedTimeline`
    (:`Update`
      (bind _playerchar (message `/Game/Blueprints/Interfaces/INT_PlayerCharacter.PlayerCharRef` (`GameplayStatics.GetPlayerCharacter` 0)))
      (`self.GetRemainingText`)
      (bind _returnvalue (`MainCharacter.IsHoldingObject` _playerchar))
      (if _returnvalue
        (`Widget.SetVisibility` _button1hbox "Collapsed")
        (else
          (`TextBlock.SetText` (`/Game/Blueprints/UI/W_PlayerHUD.Button1Text` _playerhud) "Collect")
          (`Widget.SetVisibility` _button1hbox "Visible"))))))

(event `IsUnfocused`
  (`TimelineComponent.Stop` (`self.IsFocusedTimeline`))
  (`Widget.SetVisibility` (`/Game/Blueprints/UI/W_PlayerHUD.Button1HBox` (`/Game/Blueprints/InteractableEnvironment/BP_Reception.PlayerHUD` (`self.BPReception`))) "Collapsed"))

(event `self.Box.OnComponentBeginOverlap`
  (params (OverlappedComponent :type "PrimitiveComponent Object Reference") (OtherActor :type "Actor Object Reference") (OtherComp :type "PrimitiveComponent Object Reference") (OtherBodyIndex :type Integer) (bFromSweep :type Boolean) (SweepResult :type "HitResult Structure (by ref)"))
  (bind _playerchar (message `/Game/Blueprints/Interfaces/INT_PlayerCharacter.PlayerCharRef` OtherActor))
  (if (and (== _playerchar OtherActor) (`/Game/Blueprints/InteractableEnvironment/BP_Reception.QuestReceived` (`self.BPReception`)))
    (`self.IsFocused`)))

(event `self.Box.OnComponentEndOverlap`
  (params (OverlappedComponent :type "PrimitiveComponent Object Reference") (OtherActor :type "Actor Object Reference") (OtherComp :type "PrimitiveComponent Object Reference") (OtherBodyIndex :type Integer))
  (bind _playerchar (message `/Game/Blueprints/Interfaces/INT_PlayerCharacter.PlayerCharRef` OtherActor))
  (if (== _playerchar OtherActor)
    (`self.IsUnfocused`)))

(event `SetVariables`
  ;[1 1 1] Set in Child
)

(event `GetRemainingText`
  ;[1 1 1] Set in Child
)

(fn `RotateToPlayer`
  (params (UIToRotate :type "WidgetComponent Object Reference"))
  (bind _returnvalue (`GameplayStatics.GetPlayerCharacter` 0))
  (`/Engine/EditorBlueprintResources/StandardMacros.IsValid` _returnvalue
    (:`Is Valid`
      (bind _playerchar (message `/Game/Blueprints/Interfaces/INT_PlayerCharacter.PlayerCharRef` _returnvalue))
      (`SceneComponent.K2_SetWorldRotation` UIToRotate (`KismetMathLibrary.FindLookAtRotation` (`SceneComponent.K2_GetComponentLocation` UIToRotate) (`SceneComponent.K2_GetComponentLocation` (`/Game/Blueprints/BP_MainCharacter.Camera` _playerchar))) false false))))

(fn `SetImage`)

(fn `SetRemainingText`
  (params (Limit :type Integer))
  (`TextBlock.SetText` (`/Game/Blueprints/UI/W_ContainerIndicator.RemainingText` (`self.ContainerIndicator`)) (`|FormatText` "Uses: {Available}/{Limit}" (`KismetArrayLibrary.Array_Length` (`self.CurrentCreatures`)) Limit)))

(fn `UserConstructionScript`)