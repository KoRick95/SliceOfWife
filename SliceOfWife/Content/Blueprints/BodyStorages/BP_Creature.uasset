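; BP_Creature is a creature pawn that shows a "Pick up" HUD prompt while the player overlaps its box collider.
; A focus timeline repeatedly checks that the player's hands are empty before showing the prompt through BP_Reception's PlayerHUD.
; A self-repeating Roaming event moves it to random navigable points with pauses, but nothing here starts it.
; Spawn-location capture and the initial walk-speed setup are disconnected.
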(event `self.ReceiveBeginPlay`
  (bind _returnvalue (`GameplayStatics.GetActorOfClass` "/Game/Blueprints/InteractableEnvironment/BP_Reception.BP_Reception_C"))
  (set `self.BPReception` _returnvalue))

(event `IsFocused`
  (bind _playerhud (`/Game/Blueprints/InteractableEnvironment/BP_Reception.PlayerHUD` (`self.BPReception`)))
  (`Timeline|IsFocusedTimeline`
    (:`Update`
      (bind _playerchar (message `/Game/Blueprints/Interfaces/INT_PlayerCharacter.PlayerCharRef` (`GameplayStatics.GetPlayerCharacter` 0)))
      (bind _returnvalue (`MainCharacter.IsHoldingObject` _playerchar))
      (if (not _returnvalue)
        (`TextBlock.SetText` (`/Game/Blueprints/UI/W_PlayerHUD.Button1Text` _playerhud) "Pick up")
        (`Widget.SetVisibility` (`/Game/Blueprints/UI/W_PlayerHUD.Button1HBox` _playerhud) "Visible")))))

(event `IsUnfocused`
  (`TimelineComponent.Stop` (`self.IsFocusedTimeline`))
  (`Widget.SetVisibility` (`/Game/Blueprints/UI/W_PlayerHUD.Button1HBox` (`/Game/Blueprints/InteractableEnvironment/BP_Reception.PlayerHUD` (`self.BPReception`))) "Collapsed"))

(event `Roaming`
  (if (not (`self.IsRoaming`))
    (`|AIMoveTo` (`self.FloatingPawnMovement`) self (`NavigationSystemV1.K2_GetRandomLocationInNavigableRadius` (`self.SpawnLocation`) (`self.RoamRadius`) null null) null 70.0
      (:`then`
        (set `self.IsRoaming` true))
      (:`OnSuccess`
        (`KismetSystemLibrary.Delay` (`KismetMathLibrary.RandomFloatInRange` 2.0 5.0))
        (set `self.IsRoaming` false)
        (`self.Roaming`))
      (:`OnFail`
        (`KismetSystemLibrary.PrintString` "Failed FloatingPawnMovementRoaming")))))

(event `self.BoxCollider.OnComponentBeginOverlap`
  (params (OverlappedComponent :type "PrimitiveComponent Object Reference") (OtherActor :type "Actor Object Reference") (OtherComp :type "PrimitiveComponent Object Reference") (OtherBodyIndex :type Integer) (bFromSweep :type Boolean) (SweepResult :type "HitResult Structure (by ref)"))
  (bind _playerchar (message `/Game/Blueprints/Interfaces/INT_PlayerCharacter.PlayerCharRef` OtherActor))
  (if (== _playerchar OtherActor)
    (`self.IsFocused`)))

(event `self.BoxCollider.OnComponentEndOverlap`
  (params (OverlappedComponent :type "PrimitiveComponent Object Reference") (OtherActor :type "Actor Object Reference") (OtherComp :type "PrimitiveComponent Object Reference") (OtherBodyIndex :type Integer))
  (bind _playerchar (message `/Game/Blueprints/Interfaces/INT_PlayerCharacter.PlayerCharRef` OtherActor))
  (if (== _playerchar OtherActor)
    (`self.IsUnfocused`)))

(fn `SetMovementState`
  (params (MovementState :type "/Game/Blueprints/Enums/E_MovementState Enum" :default "NewEnumerator0"))
  (bind _walkspeed (`self.WalkSpeed`))
  (set `FloatingPawnMovement.MaxSpeed` (select `/Game/Blueprints/Enums/E_MovementState` MovementState :`NewEnumerator1` _walkspeed :`NewEnumerator2` (* _walkspeed (`self.SprintSpeedMultiplier`))) (`self.FloatingPawnMovement`)))

(fn `UserConstructionScript`)