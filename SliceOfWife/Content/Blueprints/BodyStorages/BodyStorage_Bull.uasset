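; Bull variant of a body storage container that adds the bull creature to its creature pool on BeginPlay.
; It sets the indicator to the bull sprite and, when limited, takes its body count and remaining text from the game instance's bull limit, otherwise showing unlimited uses.
; Tick drives a self-resetting DoOnce with a random delay to play periodic bull huffs at the storage's location.
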(event `self.ReceiveBeginPlay`
  (`parent.ReceiveBeginPlay`)
  (`KismetArrayLibrary.Array_AddUnique` (`self.CreaturePool`) "/Game/Blueprints/BodyStorages/Creature_Bull.Creature_Bull_C"))

(event `self.ReceiveTick`
  (params (DeltaSeconds :type "Float (single-precision)"))
  (`parent.ReceiveTick` 0.0)
  (`/Engine/EditorBlueprintResources/StandardMacros.DoOnce` false :!label _label
    (:`Completed`
      (`KismetSystemLibrary.Delay` (`KismetMathLibrary.RandomFloatInRange` 4.0 8.0))
      (`GameplayStatics.SpawnSoundAtLocation` "/Game/Assets/SFX/Cues/BullHuff.BullHuff" (`SceneComponent.K2_GetComponentLocation` (`self.DefaultSceneRoot`)) (struct) 1.0 1.0 0.0 "/Game/Blueprints/Sounds/Pidgeon.Pidgeon" null)
      (goto _label :!via `Reset`))))

(event `self.SetVariables`
  (`Image.SetBrush` (`/Game/Blueprints/UI/W_ContainerIndicator.Img_ContainerType` (`self.ContainerIndicator`)) (make `SlateBrush` (32.0 32.0) (struct) (struct :`SpecifiedColor` (struct :`R` 1.0 :`G` 1.0 :`B` 1.0 :`A` 1.0) :`ColorUseRule` "UseColor_Specified") "/Game/Assets/Sprites/Sprite_Bull.Sprite_Bull"))
  (if (`self.IsLimited`)
    (set `self.MaxBodyCount` (`/Game/Blueprints/VN_GameInstance.MaxBullLimit` (`self.VN_GameInstance`)))
    (else
      (`TextBlock.SetText` (`/Game/Blueprints/UI/W_ContainerIndicator.RemainingText` (`self.ContainerIndicator`)) "Uses: ∞"))))

(event `self.GetRemainingText`
  (if (`self.IsLimited`)
    (`self.SetRemainingText` (`/Game/Blueprints/VN_GameInstance.MaxBullLimit` (`self.VN_GameInstance`)))))

(fn `UserConstructionScript`
  (`parent.UserConstructionScript`))