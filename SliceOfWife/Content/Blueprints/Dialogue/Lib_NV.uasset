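; Function library for dialogue text that converts a Text into Rich Text style markup, returned as both String and Text.
; ToTargetText prefixes a Normal tag when the text lacks an opening tag and can wrap the content after the first tag in quotes.
; It then closes each style by inserting a closing tag before every opening bracket, chopping the leading extra and closing the last one, so source text needs only opening tags.
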(fn `ToTargetText`
  (params (InText :type Text) (AddQuotes :type Boolean))
  (returns (OutString :type String) (OutText :type Text))
  (locals (ProcessedString :type String))
  (bind _processedstring (`local.ProcessedString`))
  (bind (_lefts _rights) (`KismetStringLibrary.Split` (`local.ProcessedString`) ">"))
  (set `local.ProcessedString` (`KismetTextLibrary.Conv_TextToString` InText))
  (`|ExecutionSequence`
    (:`then_0`
      ;[1 1 1] Make sure text starts with an opening tag
      (if (not (`KismetStringLibrary.StartsWith` (`local.ProcessedString`) "<"))
        (set `local.ProcessedString` (`KismetStringLibrary.Concat_StrStr` "<Normal>" (`local.ProcessedString`)))))
    (:`then_1`
      ;[1 1 1] Add Quotes
      (if AddQuotes
        (set `local.ProcessedString` (`KismetStringLibrary.Concat_StrStr` _lefts ">\"" _rights "\""))))
    (:`then_2`
      ;[1 1 1] Close all tags
      (`KismetStringLibrary.ReplaceInline` (`local.ProcessedString`) "<" "</><")
      (set `local.ProcessedString` (`KismetStringLibrary.RightChop` (`local.ProcessedString`) 3)))
    (:`then_4`
      ;[1 1 1] Close last style tag
      (set `local.ProcessedString` (`KismetStringLibrary.Concat_StrStr` (`local.ProcessedString`) "</>")))
    (:`then_5`
      (return _processedstring (`KismetTextLibrary.Conv_StringToText` _processedstring)))))