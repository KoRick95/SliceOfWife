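; Player character Blueprint that handles mouse look and interaction with BP_Reception dialogue objects.
; BoxCollider overlaps set or clear the CurrentInteractable struct and toggle the reception's focus.
; The Interact input calls the character's own Interact, then the stored reception's when usable.
; Mouse axes apply local yaw to Cam and Mesh and pitch to SpringArm, while BeginPlay sets camera-manager pitch limits.
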(event `self.ReceiveBeginPlay`
  (`self.Set Cam Min Max`)
  (set `self.Collider_var` (`self.CapsuleComponent`)))

(event `self.BoxCollider.OnComponentBeginOverlap`
  (params (OverlappedComponent :type "PrimitiveComponent Object Reference") (OtherActor :type "Actor Object Reference") (OtherComp :type "PrimitiveComponent Object Reference") (OtherBodyIndex :type Integer) (bFromSweep :type Boolean) (SweepResult :type "HitResult Structure (by ref)"))
  ;[1 1 1] If player is near dialogue object, allow interaction
  (if (`KismetMathLibrary.ClassIsChildOf` (`GameplayStatics.GetObjectClass` OtherActor) "/Game/Blueprints/InteractableEnvironment/BP_Reception.BP_Reception_C")
    (bind _asbp_reception (cast `/Game/Blueprints/InteractableEnvironment/BP_Reception` OtherActor))
    (set `self.CurrentInteractable` (make `/Game/Blueprints/Structures/ST_Interactable` true false null _asbp_reception))
    (`/Game/Blueprints/InteractableEnvironment/BP_Reception.IsFocused` _asbp_reception)))

(event `self.BoxCollider.OnComponentEndOverlap`
  (params (OverlappedComponent :type "PrimitiveComponent Object Reference") (OtherActor :type "Actor Object Reference") (OtherComp :type "PrimitiveComponent Object Reference") (OtherBodyIndex :type Integer))
  (bind (_currentinteractable_canuse _currentinteractable_isbodypart _currentinteractable_soul _currentinteractable_reception) (break `/Game/Blueprints/Structures/ST_Interactable` (`self.CurrentInteractable`)))
  ;[1 1 1] If player is no longer near dialogue object, disable interaction
  (if (== OtherActor _currentinteractable_reception)
    (`/Game/Blueprints/InteractableEnvironment/BP_Reception.IsUnfocused` _currentinteractable_reception)
    (set `self.CurrentInteractable` (make `/Game/Blueprints/Structures/ST_Interactable` false))))

(event `InputAction|Interact`
  (params (Key :type "Key Structure"))
  (bind (_currentinteractable_canuse _currentinteractable_isbodypart _currentinteractable_soul _currentinteractable_reception) (break `/Game/Blueprints/Structures/ST_Interactable` (`self.CurrentInteractable`)))
  (:`Pressed`
    (`self.Interact`)
    (if _currentinteractable_canuse
      (`/Game/Blueprints/InteractableEnvironment/BP_Reception.Interact` _currentinteractable_reception))))

(event `InputAxis|MouseLookRight`
  (params (AxisValue :type "Float (single-precision)"))
  (`SceneComponent.K2_AddLocalRotation` (`self.Cam`) (`KismetMathLibrary.MakeRotator` 0.0 0.0 AxisValue) false false)
  (`SceneComponent.K2_AddLocalRotation` (`self.Mesh`) (`KismetMathLibrary.MakeRotator` 0.0 0.0 AxisValue) false false))

(event `InputAxis|MouseLookUp`
  (params (AxisValue :type "Float (single-precision)"))
  (`SceneComponent.K2_AddLocalRotation` (`self.SpringArm`) (`KismetMathLibrary.MakeRotator` 0.0 AxisValue) false false))

(fn `Set Cam Min Max`
  (bind _returnvalue (`GameplayStatics.GetPlayerCameraManager` 0))
  (set `PlayerCameraManager.ViewPitchMin` -10.0 _returnvalue)
  (set `PlayerCameraManager.ViewPitchMax` 10.0 _returnvalue))

(fn `UserConstructionScript`)