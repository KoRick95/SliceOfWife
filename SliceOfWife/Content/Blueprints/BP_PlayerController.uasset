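; Player controller Blueprint that toggles between the menu and the dialogue view during gameplay.
; On release of the Toggle Game/Menu input, it gets the menu widget from BP_GameInstance and proceeds only if that widget reports being in game.
; The widget's canvas panel visibility serves as the toggle state: HitTestInvisible shows the menu, any other value shows the dialogue widget.
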(event `InputAction|Toggle Game/Menu`
  (params (Key :type "Key Structure"))
  (bind _menuwidget (`/Game/Blueprints/BP_GameInstance.MenuWidget` (cast `/Game/Blueprints/BP_GameInstance` (`GameplayStatics.GetGameInstance`) :!pure true)))
  (:`Released`
    (if (`/Game/Blueprints/UI/W_Menu.IsInGame` _menuwidget)
      (if (`|EnumEquality` (`Widget.GetVisibility` (`/Game/Blueprints/UI/W_Menu.CanvasPanel_0` _menuwidget)) "HitTestInvisible")
        (`/Game/Blueprints/UI/W_Menu.ShowMenuWidget` _menuwidget 1)
        (else
          (`/Game/Blueprints/UI/W_Menu.ShowDialogueWidget` _menuwidget))))))

(fn `UserConstructionScript`)