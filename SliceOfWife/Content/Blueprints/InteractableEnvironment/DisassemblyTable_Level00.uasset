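; Level 00 disassembly table that links its charge progress to the first quest objective.
; After running the parent Tick, it polls its Charge every frame against a hardcoded threshold rather than the unused MaxCharge variable.
; Once the threshold is reached, it sets the objective 1 completion flag on the quest HUD through the BPReception reference's player HUD, repeating the write each frame while the condition holds.
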(event `self.ReceiveTick`
  (params (DeltaSeconds :type "Float (single-precision)"))
  (`parent.ReceiveTick` DeltaSeconds)
  (`self.CheckDisassembly`))

(event `CheckDisassembly`
  (if (>= (`self.Charge`) 4.0)
    (set `/Game/Blueprints/UI/W_QuestHUD.CompleteObejctive1` true (`/Game/Blueprints/UI/W_PlayerHUD.W_QuestHUD` (`/Game/Blueprints/InteractableEnvironment/BP_Reception.PlayerHUD` (`self.BPReception`))))))

(fn `UserConstructionScript`
  (`parent.UserConstructionScript`))