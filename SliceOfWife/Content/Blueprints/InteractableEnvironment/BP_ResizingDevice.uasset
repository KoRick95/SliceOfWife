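; BP_ResizingDevice is an interactable device where the player can place a valid held object and later extract it, presumably for resizing.
; Player overlap runs a timeline that keeps updating Place or Extract HUD prompts through BP_Reception, based on occupancy and the held object.
; Tick updates the timer, shows the usable indicator when a valid object is held and the device is empty, and rotates visible indicator and timer widgets toward the player camera.
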(event `self.ReceiveTick`
  (params (DeltaSeconds :type "Float (single-precision)"))
  (bind _returnvalue (`GameplayStatics.GetPlayerCharacter` 0))
  (bind _usableindicator (`self.UsableIndicator`))
  (`self.UpdateTimer`)
  (if (`self.IndicatorVisible`)
    (`self.RotateToPlayer` (`self.UsableIndicator`)))
  (if (`self.TimerVisible`)
    (`self.RotateToPlayer` (`self.Timer`)))
  (bind _returnvalue_2 (`self.IsOccupied`))
  (if (not _returnvalue_2)
    (`/Engine/EditorBlueprintResources/StandardMacros.IsValid` _returnvalue
      (:`Is Valid`
        (bind _playerchar (message `/Game/Blueprints/Interfaces/INT_PlayerCharacter.PlayerCharRef` _returnvalue))
        (bind _returnvalue_3 (`self.IsValidObject` (`MainCharacter.HeldObject` _playerchar)))
        (if _returnvalue_3
          (bind _output_get (set `self.IndicatorVisible` true))
          (`SceneComponent.SetVisibility` _usableindicator _output_get false)
          (else
            (bind _output_get_2 (set `self.IndicatorVisible` false))
            (`SceneComponent.SetVisibility` _usableindicator _output_get_2 false)))))))

(event `self.ReceiveBeginPlay`
  (`self.SetReferences`))

(event `IsFocused`
  (bind _playerhud (`/Game/Blueprints/InteractableEnvironment/BP_Reception.PlayerHUD` (`self.BP_Reception`)))
  (bind _playerhud_2 (`/Game/Blueprints/InteractableEnvironment/BP_Reception.PlayerHUD` (`self.BP_Reception`)))
  (`Timeline|IsFocusedTimeline`
    (:`Update`
      (bind _returnvalue (`self.IsOccupied`))
      (if _returnvalue
        (`TextBlock.SetText` (`/Game/Blueprints/UI/W_PlayerHUD.Button2Text` _playerhud) "Extract")
        (`Widget.SetVisibility` (`/Game/Blueprints/UI/W_PlayerHUD.Button2HBox` _playerhud) "Visible")
        (`Widget.SetVisibility` (`/Game/Blueprints/UI/W_PlayerHUD.Button1HBox` _playerhud) "Collapsed")
        (bind _output_get (set `self.TimerVisible` true))
        (`SceneComponent.SetVisibility` (`self.Timer`) _output_get false)
        (bind _output_get_2 (set `self.IndicatorVisible` false))
        (`SceneComponent.SetVisibility` (`self.UsableIndicator`) _output_get_2 false)
        (else
          (bind _output_get_3 (set `self.TimerVisible` false))
          (`SceneComponent.SetVisibility` (`self.Timer`) _output_get_3 false)
          (bind _playerchar (message `/Game/Blueprints/Interfaces/INT_PlayerCharacter.PlayerCharRef` (`GameplayStatics.GetPlayerCharacter` 0)))
          (bind _returnvalue_2 (`self.IsValidObject` (`MainCharacter.HeldObject` _playerchar)))
          (if _returnvalue_2
            (`TextBlock.SetText` (`/Game/Blueprints/UI/W_PlayerHUD.Button1Text` _playerhud_2) "Place")
            (`Widget.SetVisibility` (`/Game/Blueprints/UI/W_PlayerHUD.Button1HBox` _playerhud_2) "Visible")
            (bind _output_get_4 (set `self.IndicatorVisible` true))
            (`SceneComponent.SetVisibility` (`self.UsableIndicator`) _output_get_4 false)
            (else
              (bind _output_get_5 (set `self.IndicatorVisible` false))
              (`SceneComponent.SetVisibility` (`self.UsableIndicator`) _output_get_5 false))))))))

(event `IsUnfocused`
  (`TimelineComponent.Stop` (`self.IsFocusedTimeline`))
  (`Widget.SetVisibility` (`/Game/Blueprints/UI/W_PlayerHUD.Button1HBox` (`/Game/Blueprints/InteractableEnvironment/BP_Reception.PlayerHUD` (`self.BP_Reception`))) "Collapsed")
  (`Widget.SetVisibility` (`/Game/Blueprints/UI/W_PlayerHUD.Button2HBox` (`/Game/Blueprints/InteractableEnvironment/BP_Reception.PlayerHUD` (`self.BP_Reception`))) "Collapsed"))

(event `self.SkeletalMesh.OnComponentBeginOverlap`
  (params (OverlappedComponent :type "PrimitiveComponent Object Reference") (OtherActor :type "Actor Object Reference") (OtherComp :type "PrimitiveComponent Object Reference") (OtherBodyIndex :type Integer) (bFromSweep :type Boolean) (SweepResult :type "HitResult Structure (by ref)"))
  (bind _playerchar (message `/Game/Blueprints/Interfaces/INT_PlayerCharacter.PlayerCharRef` OtherActor))
  (if (== _playerchar OtherActor)
    (`self.IsFocused`)))

(event `self.SkeletalMesh.OnComponentEndOverlap`
  (params (OverlappedComponent :type "PrimitiveComponent Object Reference") (OtherActor :type "Actor Object Reference") (OtherComp :type "PrimitiveComponent Object Reference") (OtherBodyIndex :type Integer))
  (bind _playerchar (message `/Game/Blueprints/Interfaces/INT_PlayerCharacter.PlayerCharRef` OtherActor))
  (if (== _playerchar OtherActor)
    (`self.IsUnfocused`)))

(fn `RotateToPlayer`
  (params (UIToRotate :type "WidgetComponent Object Reference"))
  (bind _returnvalue (`GameplayStatics.GetPlayerCharacter` 0))
  (`/Engine/EditorBlueprintResources/StandardMacros.IsValid` _returnvalue
    (:`Is Valid`
      (bind _playerchar (message `/Game/Blueprints/Interfaces/INT_PlayerCharacter.PlayerCharRef` _returnvalue))
      (`SceneComponent.K2_SetWorldRotation` UIToRotate (`KismetMathLibrary.FindLookAtRotation` (`SceneComponent.K2_GetComponentLocation` UIToRotate) (`SceneComponent.K2_GetComponentLocation` (`/Game/Blueprints/BP_MainCharacter.Camera` _playerchar))) false false))))

(fn `SetReferences`
  (bind _returnvalue (`GameplayStatics.GetActorOfClass` "/Game/Blueprints/InteractableEnvironment/BP_Reception.BP_Reception_C"))
  (set `self.BP_Reception` _returnvalue)
  (set `/Game/Blueprints/UI/W_CircleProgressBar.BP_ResizingDevice` self (cast `/Game/Blueprints/UI/W_CircleProgressBar` (`WidgetComponent.GetUserWidgetObject` (`self.Timer`)) :!pure true)))

(fn `UserConstructionScript`)