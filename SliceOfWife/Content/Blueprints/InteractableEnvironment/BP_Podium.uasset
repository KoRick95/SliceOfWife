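; BP_Podium is an interactable podium that shows an "Animate" button prompt while the player stands in its overlap area.
; Player overlap starts and stops a timeline, used as a per-frame update while focused.
; Each update either shows the prompt on the HUD held by BP_Reception or, if Animated is set, calls Reception's UpdateQuest.
; Leaving the area stops the timeline and collapses the prompt.
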(event `self.ReceiveBeginPlay`
  ;[1 1 1] Set a reference to Reception on startup
  (bind _returnvalue (`GameplayStatics.GetActorOfClass` "/Game/Blueprints/InteractableEnvironment/BP_Reception.BP_Reception_C"))
  (set `self.BPReception` _returnvalue))

(event `IsFocused`
  (bind _playerhud (`/Game/Blueprints/InteractableEnvironment/BP_Reception.PlayerHUD` (`self.BPReception`)))
  (`Timeline|IsFocusedTimeline`
    (:`Update`
      (if (`self.Animated`)
        (`/Game/Blueprints/InteractableEnvironment/BP_Reception.UpdateQuest` (`self.BPReception`))
        (else
          (`TextBlock.SetText` (`/Game/Blueprints/UI/W_PlayerHUD.Button2Text` _playerhud) "Animate")
          (`Widget.SetVisibility` (`/Game/Blueprints/UI/W_PlayerHUD.Button2VerticalBox` _playerhud) "Visible"))))))

(event `IsUnfocused`
  (`TimelineComponent.Stop` (`self.IsFocusedTimeline`))
  (`Widget.SetVisibility` (`/Game/Blueprints/UI/W_PlayerHUD.Button2VerticalBox` (`/Game/Blueprints/InteractableEnvironment/BP_Reception.PlayerHUD` (`self.BPReception`))) "Collapsed"))

(event `self.Podium.OnComponentBeginOverlap`
  (params (OverlappedComponent :type "PrimitiveComponent Object Reference") (OtherActor :type "Actor Object Reference") (OtherComp :type "PrimitiveComponent Object Reference") (OtherBodyIndex :type Integer) (bFromSweep :type Boolean) (SweepResult :type "HitResult Structure (by ref)"))
  (bind _playerchar (message `/Game/Blueprints/Interfaces/INT_PlayerCharacter.PlayerCharRef` OtherActor))
  (if (== _playerchar OtherActor)
    (`self.IsFocused`)))

(event `self.Podium.OnComponentEndOverlap`
  (params (OverlappedComponent :type "PrimitiveComponent Object Reference") (OtherActor :type "Actor Object Reference") (OtherComp :type "PrimitiveComponent Object Reference") (OtherBodyIndex :type Integer))
  (bind _playerchar (message `/Game/Blueprints/Interfaces/INT_PlayerCharacter.PlayerCharRef` OtherActor))
  (if (== _playerchar OtherActor)
    (`self.IsUnfocused`)))

(fn `UserConstructionScript`)