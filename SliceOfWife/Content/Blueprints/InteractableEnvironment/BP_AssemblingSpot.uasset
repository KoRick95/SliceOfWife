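; Body-part slot on the assembly table that shows whether it can take the player's held object or needs sewing.
; Tick turns the sew image and usable indicator toward the player's camera, showing the indicator when the held object can be dropped.
; Player overlap runs a focus timeline that updates HUD Place/Sew prompts and recolours a dynamic decal by occupied and sewn state.
; Empty-slot colour depends on whether the spot is optional.
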(event `self.ReceiveTick`
  (params (DeltaSeconds :type "Float (single-precision)"))
  (bind _usableindicator (`self.UsableIndicator`))
  (`self.RotateTowardsPlayer` (`self.SewImage`))
  (bind _playerchar (message `/Game/Blueprints/Interfaces/INT_PlayerCharacter.PlayerCharRef` (`GameplayStatics.GetPlayerCharacter` 0)))
  (bind _returnvalue (`self.CanDropToTable` (`MainCharacter.HeldObject` _playerchar)))
  (if _returnvalue
    (`SceneComponent.SetVisibility` _usableindicator true false)
    (`self.RotateTowardsPlayer` (`self.UsableIndicator`))
    (else
      (`SceneComponent.SetVisibility` _usableindicator false false))))

(event `self.ReceiveBeginPlay`
  (bind _decal (`self.Decal`))
  (`self.SetReferences`)
  (bind _returnvalue (`DecalComponent.CreateDynamicMaterialInstance` _decal))
  (bind _output_get (set `self.DMI_Decal` _returnvalue))
  (`DecalComponent.SetDecalMaterial` _decal _output_get)
  (`self.SetInitialDecalColour`))

(event `IsFocused`
  (bind _dmi_decal (`self.DMI_Decal`))
  (bind _dmi_decal_2 (`self.DMI_Decal`))
  (bind _playerhud (`/Game/Blueprints/InteractableEnvironment/BP_Reception.PlayerHUD` (`self.BP_Reception`)))
  (bind _playerhud_2 (`/Game/Blueprints/InteractableEnvironment/BP_Reception.PlayerHUD` (`self.BP_Reception`)))
  (`Timeline|IsFocusedTimeline`
    (:`Update`
      (bind _returnvalue (`self.IsOccupied`))
      (if _returnvalue
        (bind _returnvalue_2 (`self.IsBodyPartSewn`))
        (if _returnvalue_2
          (`MaterialInstanceDynamic.SetVectorParameterValue` _dmi_decal_2 "Base Colour" (struct :`G` 0.005536 :`B` 1.0 :`A` 1.0))
          (`MaterialInstanceDynamic.SetScalarParameterValue` _dmi_decal_2 "Emiss Intensity" 100.0)
          (`SceneComponent.SetVisibility` (`self.SewImage`) false false)
          (else
            (`MaterialInstanceDynamic.SetVectorParameterValue` _dmi_decal "Base Colour" (struct :`R` 1.0 :`G` 0.943703 :`A` 1.0))
            (`MaterialInstanceDynamic.SetScalarParameterValue` _dmi_decal "Emiss Intensity" 1000.0)
            (bind _returnvalue_3 (`AssemblingTable.IsCentreOccupied` (`self.BP_AssemblyTable`)))
            (if _returnvalue_3
              (`TextBlock.SetText` (`/Game/Blueprints/UI/W_PlayerHUD.Button2Text` _playerhud_2) "Sew")
              (`Widget.SetVisibility` (`/Game/Blueprints/UI/W_PlayerHUD.Button2HBox` _playerhud_2) "Visible")
              (`Widget.SetVisibility` (`/Game/Blueprints/UI/W_PlayerHUD.Button1HBox` _playerhud_2) "Collapsed"))))
        (else
          (`self.SetInitialDecalColour`)
          (bind _playerchar (message `/Game/Blueprints/Interfaces/INT_PlayerCharacter.PlayerCharRef` (`GameplayStatics.GetPlayerCharacter` 0)))
          (bind _returnvalue_4 (`self.CanDropToTable` (`MainCharacter.HeldObject` _playerchar)))
          (if _returnvalue_4
            (`TextBlock.SetText` (`/Game/Blueprints/UI/W_PlayerHUD.Button1Text` _playerhud) "Place")
            (`Widget.SetVisibility` (`/Game/Blueprints/UI/W_PlayerHUD.Button1HBox` _playerhud) "Visible")))))))

(event `IsUnfocused`
  (`TimelineComponent.Stop` (`self.IsFocusedTimeline`))
  (`Widget.SetVisibility` (`/Game/Blueprints/UI/W_PlayerHUD.Button1HBox` (`/Game/Blueprints/InteractableEnvironment/BP_Reception.PlayerHUD` (`self.BP_Reception`))) "Collapsed")
  (`Widget.SetVisibility` (`/Game/Blueprints/UI/W_PlayerHUD.Button2HBox` (`/Game/Blueprints/InteractableEnvironment/BP_Reception.PlayerHUD` (`self.BP_Reception`))) "Collapsed"))

(event `self.BoxOverlapCollider.OnComponentBeginOverlap`
  (params (OverlappedComponent :type "PrimitiveComponent Object Reference") (OtherActor :type "Actor Object Reference") (OtherComp :type "PrimitiveComponent Object Reference") (OtherBodyIndex :type Integer) (bFromSweep :type Boolean) (SweepResult :type "HitResult Structure (by ref)"))
  (bind _playerchar (message `/Game/Blueprints/Interfaces/INT_PlayerCharacter.PlayerCharRef` OtherActor))
  (if (== _playerchar OtherActor)
    (`self.IsFocused`)))

(event `self.BoxOverlapCollider.OnComponentEndOverlap`
  (params (OverlappedComponent :type "PrimitiveComponent Object Reference") (OtherActor :type "Actor Object Reference") (OtherComp :type "PrimitiveComponent Object Reference") (OtherBodyIndex :type Integer))
  (bind _playerchar (message `/Game/Blueprints/Interfaces/INT_PlayerCharacter.PlayerCharRef` OtherActor))
  (if (== _playerchar OtherActor)
    (`self.IsUnfocused`)))

(fn `RotateTowardsPlayer`
  (params (Indicator :type "WidgetComponent Object Reference"))
  (bind _playerchar (message `/Game/Blueprints/Interfaces/INT_PlayerCharacter.PlayerCharRef` (`GameplayStatics.GetPlayerCharacter` 0)))
  (`SceneComponent.K2_SetWorldRotation` Indicator (`KismetMathLibrary.FindLookAtRotation` (`SceneComponent.K2_GetComponentLocation` Indicator) (`SceneComponent.K2_GetComponentLocation` (`/Game/Blueprints/BP_MainCharacter.Camera` _playerchar))) false false))

(fn `SetInitialDecalColour`
  (bind _dmi_decal (`self.DMI_Decal`))
  (bind _dmi_decal_2 (`self.DMI_Decal`))
  (if (`self.IsOptional`)
    (`MaterialInstanceDynamic.SetVectorParameterValue` _dmi_decal_2 "Base Colour" (struct :`G` 0.005536 :`B` 1.0 :`A` 1.0))
    (`MaterialInstanceDynamic.SetScalarParameterValue` _dmi_decal_2 "Emiss Intensity" 1000.0)
    (else
      (`MaterialInstanceDynamic.SetVectorParameterValue` _dmi_decal "Base Colour" (struct :`R` 0.921875 :`G` 0.004801 :`B` 0.004801 :`A` 1.0))
      (`MaterialInstanceDynamic.SetScalarParameterValue` _dmi_decal "Emiss Intensity" 1000.0))))

(fn `SetReferences`
  (bind _returnvalue (`GameplayStatics.GetActorOfClass` "/Game/Blueprints/InteractableEnvironment/BP_Reception.BP_Reception_C"))
  (set `self.BP_Reception` _returnvalue)
  (bind _returnvalue_2 (`GameplayStatics.GetActorOfClass` "/Game/Blueprints/InteractableEnvironment/BP_AssemblyTable.BP_AssemblyTable_C"))
  (set `self.BP_AssemblyTable` _returnvalue_2))

(fn `UserConstructionScript`)