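; Level 00 variant of the resizing device interactable, extending a parent device with a quest hook.
; Each tick it gets the player's held object through a player character reference message and shows the usable indicator only when that object is valid.
; When focused, it marks objective 2 complete on the quest HUD, reached through BPReception's player HUD, and refreshes the checkmarks.
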(event `self.ReceiveTick`
  (params (DeltaSeconds :type "Float (single-precision)"))
  (bind _returnvalue (`GameplayStatics.GetPlayerCharacter` 0))
  (bind _usableindicator (`self.UsableIndicator`))
  (`parent.ReceiveTick` DeltaSeconds)
  (`/Engine/EditorBlueprintResources/StandardMacros.IsValid` _returnvalue
    (:`Is Valid`
      (bind _playerchar (message `/Game/Blueprints/Interfaces/INT_PlayerCharacter.PlayerCharRef` _returnvalue))
      (bind _returnvalue_2 (`self.IsValidObject` (`MainCharacter.HeldObject` _playerchar)))
      (if _returnvalue_2
        (bind _output_get (set `self.IndicatorVisible` true))
        (`SceneComponent.SetVisibility` _usableindicator _output_get false)
        (else
          (bind _output_get_2 (set `self.IndicatorVisible` false))
          (`SceneComponent.SetVisibility` _usableindicator _output_get_2 false))))))

(event `self.IsFocused`
  (bind _w_questhud (`/Game/Blueprints/UI/W_PlayerHUD.W_QuestHUD` (`/Game/Blueprints/InteractableEnvironment/BP_Reception.PlayerHUD` (`self.BP_Reception`))))
  (`parent.IsFocused`)
  (if true
    (set `/Game/Blueprints/UI/W_QuestHUD.CompleteObjective2` true _w_questhud)
    (`/Game/Blueprints/UI/W_QuestHUD.SetChecked` _w_questhud)))

(fn `UserConstructionScript`
  (`parent.UserConstructionScript`))