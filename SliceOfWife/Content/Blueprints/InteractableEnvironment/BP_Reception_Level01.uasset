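; Level 01 reception interactable that hands out the Aristocat quest and plays the level's opening and ending dialogues.
; SceneLaunch starts the intro dialogue through the game instance's dialogue widget, flags the quest as received and switches the objective sprite to the quest icon.
; EndSceneLaunch plays the closing dialogue and turns off the quest notification.
; PickLocalScene supplies the scene name, while PickDialogue is left empty.
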(event `self.SceneLaunch`
  (bind _questobjective (`self.QuestObjective`))
  (`/Game/Blueprints/DialogueSystem/W_VNDialogue.StartDialogue` (`/Game/Blueprints/VN_GameInstance.GameInsDialogueWidget` (cast `/Game/Blueprints/VN_GameInstance` (`GameplayStatics.GetGameInstance`) :!pure true)) "/Game/Blueprints/Dialogue/Dlg_Level01.Dlg_Level01")
  (set `self.QuestReceived` true)
  (`SceneComponent.SetWorldScale3D` _questobjective (0.07 0.07 0.07))
  (`PaperSpriteComponent.SetSprite` _questobjective "/Game/Assets/Sprites/UI_Art/Sprite_QuestAristocat.Sprite_QuestAristocat"))

(event `self.EndSceneLaunch`
  (`/Game/Blueprints/DialogueSystem/W_VNDialogue.StartDialogue` (`/Game/Blueprints/VN_GameInstance.GameInsDialogueWidget` (cast `/Game/Blueprints/VN_GameInstance` (`GameplayStatics.GetGameInstance`) :!pure true)) "/Game/Blueprints/Dialogue/Dlg_EndLevel01.Dlg_EndLevel01")
  (set `self.ShowNotification` false)
  (`self.ToggleQuestNotification`))

(fn `PickDialogue`
  (returns (`AsDlg Dialogue` :type "DlgDialogue Object Reference"))
  (return null))

(fn `PickLocalScene`
  (returns (DialogueName :type Name))
  (return "Dlg_Level01"))

(fn `UserConstructionScript`
  (`parent.UserConstructionScript`))