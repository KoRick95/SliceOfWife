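; Reception_Level02 is the level 2 variant of an interactable reception, supplying that level's objective display and dialogue scenes.
; It creates the Objective_Level02 widget when child references are set, then forwards display and hide events to it.
; Start, end and failed-request events each launch a dialogue scene, with failure using Dlg_LevelFailed01.
; The end event also enables a notification and refreshes the quest widget.
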(event `self.SetChildReferences`
  (bind _returnvalue (`|CreateWidget` "/Game/Blueprints/UI/Objectives/Objective_Level02.Objective_Level02_C"))
  (set `self.Objective_Level02` _returnvalue))

(event `self.DisplayObjective`
  (`/Game/Blueprints/UI/Objectives/W_AristocatObjective.DisplayObjective` (`self.Objective_Level02`)))

(event `self.HideObjective`
  (`/Game/Blueprints/UI/Objectives/W_AristocatObjective.HideObjective` (`self.Objective_Level02`)))

(event `self.SceneLaunch`
  (`self.LaunchScene` "/Game/Blueprints/Dialogue/Dlg_LevelStart02.Dlg_LevelStart02"))

(event `self.EndSceneLaunch`
  (`self.LaunchScene` "/Game/Blueprints/Dialogue/Dlg_LevelEnd02.Dlg_LevelEnd02")
  (set `self.ShowNotification` true)
  (`self.RefreshQuestWidget`))

(event `self.RequestFailedSceneLaunch`
  (`self.LaunchScene` "/Game/Blueprints/Dialogue/Dlg_LevelFailed01.Dlg_LevelFailed01"))

(fn `UserConstructionScript`
  (`parent.UserConstructionScript`))