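; BP_AssemblyTable is an interactable assembly table that shows a "Place" button prompt on the player HUD while focused.
; On BeginPlay it finds BP_Reception and reaches the HUD through it, showing or collapsing the prompt from the IsFocused and IsUnfocused events.
; A ChangeCamera function blends the view to the table, but it and the return blend sit in disconnected logic, leaving the collider overlap events empty.
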(event `self.ReceiveBeginPlay`
  (bind _returnvalue (`GameplayStatics.GetActorOfClass` "/Game/Blueprints/InteractableEnvironment/BP_Reception.BP_Reception_C"))
  (set `self.BPReception` _returnvalue))

(event `IsFocused`
  (bind _playerhud (`/Game/Blueprints/InteractableEnvironment/BP_Reception.PlayerHUD` (`self.BPReception`)))
  (`TextBlock.SetText` (`/Game/Blueprints/UI/W_PlayerHUD.Button1Text` _playerhud) "Place")
  (`Widget.SetVisibility` (`/Game/Blueprints/UI/W_PlayerHUD.Button1VerticalBox` _playerhud) "Visible"))

(event `IsUnfocused`
  (`Widget.SetVisibility` (`/Game/Blueprints/UI/W_PlayerHUD.Button1VerticalBox` (`/Game/Blueprints/InteractableEnvironment/BP_Reception.PlayerHUD` (`self.BPReception`))) "Collapsed"))

(event `self.Access_Colider.OnComponentBeginOverlap`
  (params (OverlappedComponent :type "PrimitiveComponent Object Reference") (OtherActor :type "Actor Object Reference") (OtherComp :type "PrimitiveComponent Object Reference") (OtherBodyIndex :type Integer) (bFromSweep :type Boolean) (SweepResult :type "HitResult Structure (by ref)")))

(event `self.Access_Colider.OnComponentEndOverlap`
  (params (OverlappedComponent :type "PrimitiveComponent Object Reference") (OtherActor :type "Actor Object Reference") (OtherComp :type "PrimitiveComponent Object Reference") (OtherBodyIndex :type Integer)))

(fn `Change Camera`
  (`PlayerController.SetViewTargetWithBlend` (`GameplayStatics.GetPlayerController` 0) self 0.6 "VTBlend_Cubic" 0.0 false))

(fn `UserConstructionScript`)