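; Level 00 reception interactable that handles the level's start and end dialogue, currency assignment and request completion.
; Scene events pass the start or end dialogue to LaunchScene, with the end event also switching on and toggling the quest notification.
; Separate events call AssignCurrency and add the level's RequestComplete widget to the viewport.
; Construction defers to the parent class.
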(event `self.SceneLaunch`
  (`self.LaunchScene` "/Game/Blueprints/Dialogue/Dlg_LevelStart00.Dlg_LevelStart00"))

(event `self.EndSceneLaunch`
  (`self.LaunchScene` "/Game/Blueprints/Dialogue/Dlg_LevelEnd00.Dlg_LevelEnd00")
  (set `self.ShowNotification` true)
  (`self.ToggleQuestNotification`))

(event `self.GenerateCurrency`
  (`self.AssignCurrency`))

(event `self.RequestComplete`
  (bind _returnvalue (`|CreateWidget` "/Game/Blueprints/UI/Levels/RequestComplete_Level00.RequestComplete_Level00_C"))
  (`UserWidget.AddToViewport` _returnvalue 0))

(fn `UserConstructionScript`
  (`parent.UserConstructionScript`))