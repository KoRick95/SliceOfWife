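; Level 99 variant of an interactable reception that launches the level's start and end dialogue scenes and manages its objective widget.
; It fills in parent events: setting child references creates the Objective_Level99 widget, and display or hide calls pass straight through to it.
; The end scene event also turns on the notification flag and refreshes the quest widget.
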(event `self.SetChildReferences`
  (bind _returnvalue (`|CreateWidget` "/Game/Blueprints/UI/Objectives/Objective_Level99.Objective_Level99_C"))
  (set `self.Objective_Level99` _returnvalue))

(event `self.SceneLaunch`
  (`self.LaunchScene` "/Game/Blueprints/Dialogue/Dlg_Level99Start.Dlg_Level99Start"))

(event `self.EndSceneLaunch`
  (`self.LaunchScene` "/Game/Blueprints/Dialogue/Dlg_Level99End.Dlg_Level99End")
  (set `self.ShowNotification` true)
  (`self.RefreshQuestWidget`))

(event `self.DisplayObjective`
  (`/Game/Blueprints/UI/Objectives/W_AristocatObjective.DisplayObjective` (`self.Objective_Level99`)))

(event `self.HideObjective`
  (`/Game/Blueprints/UI/Objectives/W_AristocatObjective.HideObjective` (`self.Objective_Level99`)))

(fn `UserConstructionScript`
  (`parent.UserConstructionScript`))