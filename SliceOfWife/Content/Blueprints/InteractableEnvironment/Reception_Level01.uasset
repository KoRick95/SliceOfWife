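; Level 01 variant of an interactable reception that launches the level's dialogue scenes and controls its objective widget.
; It overrides parent hooks to launch separate start, end and failure scenes and to name the local dialogue scene.
; The end scene also flags a notification and refreshes the quest widget.
; It creates the Level 01 objective widget and forwards show and hide calls to it.
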(event `self.SetChildReferences`
  (bind _returnvalue (`|CreateWidget` "/Game/Blueprints/UI/Objectives/Objective_Level01.Objective_Level01_C"))
  (set `self.Objective_Level01` _returnvalue))

(event `self.SceneLaunch`
  (`self.LaunchScene` "/Game/Blueprints/Dialogue/Dlg_LevelStart01.Dlg_LevelStart01"))

(event `self.EndSceneLaunch`
  (`self.LaunchScene` "/Game/Blueprints/Dialogue/Dlg_LevelEnd02.Dlg_LevelEnd02")
  (set `self.ShowNotification` true)
  (`self.RefreshQuestWidget`))

(event `self.RequestFailedSceneLaunch`
  (`self.LaunchScene` "/Game/Blueprints/Dialogue/Dlg_LevelFailed01.Dlg_LevelFailed01"))

(event `self.DisplayObjective`
  (`/Game/Blueprints/UI/Objectives/W_AristocatObjective.DisplayObjective` (`self.Objective_Level01`)))

(event `self.HideObjective`
  (`/Game/Blueprints/UI/Objectives/W_AristocatObjective.HideObjective` (`self.Objective_Level01`)))

(fn `PickDialogue`
  (returns (`AsDlg Dialogue` :type "DlgDialogue Object Reference"))
  (return null))

(fn `PickLocalScene`
  (returns (DialogueName :type Name))
  (return "Dlg_Level01"))

(fn `UserConstructionScript`
  (`parent.UserConstructionScript`))