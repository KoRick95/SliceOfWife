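; BP_Reception is an interactable reception environment object, apparently a scene trigger that is largely stubbed out.
; SceneLaunch and focus checks both rely on PickLocalScene, which always returns an empty string, so no scene is set and RefreshInteraction reports false.
; Interact only clears SceneTriggering when already false, and the overlap handlers do nothing.
; Logic to open or advance a W_Dialogue widget with Dlg_Level01 is disconnected and never runs.
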(event `SceneLaunch`
  (bind _dialoguename (`self.PickLocalScene`))
  (if (`KismetStringLibrary.EqualEqual_StrStr` _dialoguename)
    (set `self.CancelScene` false)
    (else
      (set `/Game/Blueprints/BP_GameInstance.CurrentScene` _dialoguename (`self.GameInstance`))))
  (if (`self.CancelScene`)
    _))

(event `Interact`
  (if (not (`self.SceneTriggering`))
    (set `self.SceneTriggering` false)))

(event `IsFocused`
  (bind _interactenabled (`self.RefreshInteraction`))
  (if _interactenabled
    (cast `/Game/Blueprints/BP_MainCharacter` (`/Game/Blueprints/BP_GameInstance.PlayerActor` (`self.GameInstance`)))))

(event `IsUnfocused`)

(event `InputAction|Interact`
  (params (Key :type "Key Structure")))

(event `self.Box.OnComponentBeginOverlap`
  (params (OverlappedComponent :type "PrimitiveComponent Object Reference") (OtherActor :type "Actor Object Reference") (OtherComp :type "PrimitiveComponent Object Reference") (OtherBodyIndex :type Integer) (bFromSweep :type Boolean) (SweepResult :type "HitResult Structure (by ref)")))

(event `self.Box.OnComponentEndOverlap`
  (params (OverlappedComponent :type "PrimitiveComponent Object Reference") (OtherActor :type "Actor Object Reference") (OtherComp :type "PrimitiveComponent Object Reference") (OtherBodyIndex :type Integer))
  (if (`KismetSystemLibrary.IsValid` (`self.DialogueWidget`))
    _))

(fn `PickLocalScene`
  (returns (DialogueName :type String))
  (return ""))

(fn `RefreshInteraction`
  (returns (InteractEnabled :type Boolean))
  (bind _dialoguename (`self.PickLocalScene`))
  (if (`KismetStringLibrary.EqualEqual_StrStr` _dialoguename)
    (return false)
    (else
      (return true))))

(fn `UserConstructionScript`)