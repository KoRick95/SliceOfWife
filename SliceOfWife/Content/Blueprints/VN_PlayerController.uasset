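; Player controller for the VN game that toggles between the dialogue view and the menu.
; On release of the Toggle Game/Menu input, it gets the menu widget held by VN_GameInstance and acts only while that widget reports being in game.
; The visibility of the widget's canvas panel serves as the toggle state, selecting whether to show the menu or the dialogue widget.
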(event `InputAction|Toggle Game/Menu`
  (params (Key :type "Key Structure"))
  (bind _gameinsmenuwidget (`/Game/Blueprints/VN_GameInstance.GameInsMenuWidget` (cast `/Game/Blueprints/VN_GameInstance` (`GameplayStatics.GetGameInstance`) :!pure true)))
  (:`Released`
    (if (`/Game/Blueprints/DialogueSystem/W_VNMenu.IsInGame` _gameinsmenuwidget)
      (if (`|EnumEquality` (`Widget.GetVisibility` (`/Game/Blueprints/DialogueSystem/W_VNMenu.CanvasPanel_0` _gameinsmenuwidget)) "HitTestInvisible")
        (`/Game/Blueprints/DialogueSystem/W_VNMenu.ShowMenuWidget` _gameinsmenuwidget 1)
        (else
          (`/Game/Blueprints/DialogueSystem/W_VNMenu.ShowDialogueWidget` _gameinsmenuwidget))))))

(fn `UserConstructionScript`)