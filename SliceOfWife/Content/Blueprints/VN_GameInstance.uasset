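; VN_GameInstance is the visual novel game instance that owns persistent data, shared UI widgets and story flags.
; Init loads or creates the save, cross-links menu, dialogue, Reception and Podium, then async-loads assets for codex and gallery; Shutdown saves.
; As a dialogue participant, it answers conditions from TriggeredFlags and uses ModifyNameValue to set flags and update codex entries with notifications.
; Helpers reset state for new games and possess pawns without changing view target.
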(event `self.ReceiveInit`
  (bind _w_options (`/Game/Blueprints/DialogueSystem/W_VNMenu.W_Options` (`self.GameInsMenuWidget`)))
  (bind _w_codex (`/Game/Blueprints/DialogueSystem/W_VNMenu.W_Codex` (`self.GameInsMenuWidget`)))
  (`|ExecutionSequence`
    (:`then_0`
      ;[1 1 1] Get Persistant Data
      (bind _returnvalue (`GameplayStatics.DoesSaveGameExist` "VN_PersistantData" :!label _label))
      (if _returnvalue
        (bind _returnvalue_2 (`GameplayStatics.LoadGameFromSlot` "VN_PersistantData"))
        (set `self.PersistantData` (cast `/Game/Blueprints/DialogueSystem/VN_PersistantData` _returnvalue_2 :!pure true))
        (else
          (bind _returnvalue_3 (`GameplayStatics.CreateSaveGameObject` "/Game/Blueprints/DialogueSystem/VN_PersistantData.VN_PersistantData_C"))
          (bind _output_get (set `self.PersistantData` _returnvalue_3))
          (set `/Game/Blueprints/DialogueSystem/VN_PersistantData.ShowUnselectableOptions` false _output_get)
          (set `/Game/Blueprints/DialogueSystem/VN_PersistantData.TextSpeed` 0.035 _output_get))))
    (:`then_1`
      ;[1 1 1] Create Widgets and Initialise Options
      (bind _returnvalue_4 (`|CreateWidget` "/Game/Blueprints/DialogueSystem/W_VNMenu.W_VNMenu_C"))
      ;;[1 1 1] Set a reference to the Menu Widget for BP_Reception class
      (bind _returnvalue_5 (`GameplayStatics.GetActorOfClass` "/Game/Blueprints/InteractableEnvironment/BP_Reception.BP_Reception_C"))
      (set `/Game/Blueprints/InteractableEnvironment/BP_Reception.MenuWidget` _returnvalue_4 _returnvalue_5)
      (set `self.GameInsBPReception` _returnvalue_5)
      (set `/Game/Blueprints/InteractableEnvironment/BP_Reception.BPPodium` (stale _returnvalue_6) _returnvalue_5)
      ;;[1 1 1] Set a reference to BP_Podium class
      (bind _returnvalue_6 (`GameplayStatics.GetActorOfClass` "/Game/Blueprints/InteractableEnvironment/BP_Podium.BP_Podium_C"))
      (set `/Game/Blueprints/InteractableEnvironment/BP_Podium.MenuWidget` _returnvalue_4 _returnvalue_6)
      (set `self.GameInsBPPodium` _returnvalue_6)
      (set `/Game/Blueprints/InteractableEnvironment/BP_Podium.BPReception` _returnvalue_5 _returnvalue_6)
      (bind _output_get_2 (set `self.GameInsMenuWidget` _returnvalue_4))
      (bind _returnvalue_7 (`|CreateWidget` "/Game/Blueprints/DialogueSystem/W_VNDialogue.W_VNDialogue_C" null _output_get_2 (`/Game/Blueprints/DialogueSystem/W_VNMenu.W_History` _output_get_2) (`self.PersistantData`)))
      ;;[1 1 1] Set a ref to Reception
      (set `/Game/Blueprints/InteractableEnvironment/BP_Reception.DialogueWidget` _returnvalue_7 _returnvalue_5)
      ;;[1 1 1] Set a ref to Podium
      (set `/Game/Blueprints/InteractableEnvironment/BP_Podium.DialogueWidget` _returnvalue_7 _returnvalue_6)
      (bind _returnvalue_8 (`|CreateWidget` "/Game/Blueprints/UI/W_PlayerHUD.W_PlayerHUD_C" null (`GameplayStatics.GetPlayerPawn` 0)))
      (set `self.GameInsPlayerHUD` _returnvalue_8)
      (bind _output_get_3 (set `/Game/Blueprints/DialogueSystem/W_VNMenu.DialogueWidget` _returnvalue_7 _output_get_2))
      (set `self.GameInsDialogueWidget` _output_get_3)
      (bind _output_get_4 (set `self.GameInsOptionsWidget` _w_options))
      (set `/Game/Blueprints/DialogueSystem/W_VNOptions.DialogueWidget` (`self.GameInsDialogueWidget`) _output_get_4)
      (set `/Game/Blueprints/DialogueSystem/W_VNOptions.VNPersistantData` (`self.PersistantData`) _w_options)
      (`/Game/Blueprints/DialogueSystem/W_VNOptions.InitialiseSavedOptions` _w_options)
      (bind _output_get_5 (set `self.CodexWidget` _w_codex))
      (bind _outprimaryassetidlist (`KismetSystemLibrary.GetPrimaryAssetIdList` "CodexEntries"))
      (`AsyncActionLoadPrimaryAssetList.AsyncLoadPrimaryAssetList` _outprimaryassetidlist
        (:`Completed`
          (`/Game/Blueprints/DialogueSystem/W_VNCodex.CreateCodexButtons` _w_codex (`self.GameInsDialogueWidget`))
          (`/Game/Blueprints/DialogueSystem/W_VNCodex.CreateCodexButtons` _output_get_5 (`self.GameInsDialogueWidget`))
          (bind _returnvalue_9 (`|CreateWidget` "/Game/Blueprints/DialogueSystem/W_VNGalleryImage.W_VNGalleryImage_C" null (`self.PersistantData`)))
          (`/Game/Blueprints/DialogueSystem/W_VNGallery.CreateGalleryButtons` (`/Game/Blueprints/DialogueSystem/W_VNMenu.W_Gallery` (`self.GameInsMenuWidget`)) (`self.PersistantData`) _returnvalue_9)
          (bind _returnvalue_10 (`|CreateWidget` "/Game/Blueprints/UI/Objectives/W_AristocatObjective.W_AristocatObjective_C"))
          (set `self.GameInsObjectiveWidget` _returnvalue_10)
          (bind _outprimaryassetidlist_2 (`KismetSystemLibrary.GetPrimaryAssetIdList` "CodexImages"))
          (`AsyncActionLoadPrimaryAssetList.AsyncLoadPrimaryAssetList` _outprimaryassetidlist_2
            (:`then`
              (bind _outprimaryassetidlist_3 (`KismetSystemLibrary.GetPrimaryAssetIdList` "Characters"))
              (`AsyncActionLoadPrimaryAssetList.AsyncLoadPrimaryAssetList` _outprimaryassetidlist_3
                (:`then`
                  (bind _outprimaryassetidlist_4 (`KismetSystemLibrary.GetPrimaryAssetIdList` "Music"))
                  (`AsyncActionLoadPrimaryAssetList.AsyncLoadPrimaryAssetList` _outprimaryassetidlist_4))))))))))

(event `LoadGameInstance`
  (goto _label))

(event `self.ReceiveShutdown`
  ;[1 1 1] Save Persistant Data on Shutdown
  (`GameplayStatics.SaveGameToSlot` (`self.PersistantData`) "VN_PersistantData"))

(event `/Game/Blueprints/Interfaces/VN_SaveInterface.OnNewGame`
  (bind _buttonscrollbox (`/Game/Blueprints/DialogueSystem/W_VNCodex.ButtonScrollBox` (`self.CodexWidget`)))
  (`KismetArrayLibrary.Array_Clear` (`self.TriggeredFlags`))
  (set `self.PlayerName` "???")
  (`/Game/Blueprints/DialogueSystem/W_VNHistory.OnNewGame` (`/Game/Blueprints/DialogueSystem/W_VNMenu.W_History` (`self.GameInsMenuWidget`)))
  (`/Game/Blueprints/DialogueSystem/W_VNHistory.OnNewGame` (`self.GameInsDialogueWidget`))
  (for _index (range (`PanelWidget.GetChildrenCount` _buttonscrollbox))
    (`/Game/Blueprints/DialogueSystem/W_CodexButton.UpdateCodexDetails` (cast `/Game/Blueprints/DialogueSystem/W_CodexButton` (`PanelWidget.GetChildAt` _buttonscrollbox _index) :!pure true))))

(event `RefreshPlayerCharacter`
  (bind _returnvalue (`GameplayStatics.GetPlayerCharacter` 0))
  (bind _playerclass (`self.PlayerClass`))
  (`/Engine/EditorBlueprintResources/StandardMacros.IsValid` (`self.PlayerActor`)
    (:`Is Not Valid`
      (if (== _playerclass (`GameplayStatics.GetObjectClass` _returnvalue))
        (set `self.PlayerActor` _returnvalue)
        (else
          (bind _outactors (`GameplayStatics.GetAllActorsOfClass` _playerclass))
          (bind _output (`|GetArrayItem` _outactors))
          (`/Engine/EditorBlueprintResources/StandardMacros.IsValid` _output
            (:`Is Valid`
              (bind _aspawn (cast `Pawn` _output))
              (set `self.PlayerActor` _aspawn))))))))

(fn `CheckCondition`
  (params (Context :type "DlgContext Object Reference") (ConditionName :type Name))
  (returns (ReturnValue :type Boolean))
  (return (`KismetArrayLibrary.Array_Contains` (`self.TriggeredFlags`) ConditionName)))

(fn `CheckWidgetController`
  (`/Engine/EditorBlueprintResources/StandardMacros.IsValid` (`self.BP_WidgetController`)
    (:`Is Not Valid`
      (bind _returnvalue (`|SpawnActorFromClass` "/Game/Blueprints/BP_WidgetController.BP_WidgetController_C" (`KismetMathLibrary.MakeTransform` (0.0 0.0 0.0)) "Undefined" "OverrideRootScale" null null))
      (set `self.BP_WidgetController` _returnvalue))))

(fn `GetBoolValue`
  (params (ValueName :type Name))
  (returns (ReturnValue :type Boolean))
  (return false))

(fn `GetFloatValue`
  (params (ValueName :type Name))
  (returns (ReturnValue :type "Float (double-precision)"))
  (return 0.0))

(fn `GetIntValue`
  (params (ValueName :type Name))
  (returns (ReturnValue :type Integer))
  (return 0))

(fn `GetNameValue`
  (params (ValueName :type Name))
  (returns (ReturnValue :type Name))
  (return "None"))

(fn `GetParticipantDisplayName`
  (params (ActiveSpeaker :type Name))
  (returns (ReturnValue :type Text))
  (return ""))

(fn `GetParticipantGender`
  (returns (ReturnValue :type "ETextGender Enum"))
  (return "Masculine"))

(fn `GetParticipantIcon`
  (params (ActiveSpeaker :type Name) (ActiveSpeakerState :type Name))
  (returns (ReturnValue :type "Texture2D Object Reference"))
  (return null))

(fn `GetParticipantName`
  (returns (ReturnValue :type Name))
  (return "VNGameInstance"))

(fn `ModifyBoolValue`
  (params (ValueName :type Name) (bNewValue :type Boolean))
  (returns (ReturnValue :type Boolean))
  (return false))

(fn `ModifyFloatValue`
  (params (ValueName :type Name) (bDelta :type Boolean) (Value :type "Float (double-precision)"))
  (returns (ReturnValue :type Boolean))
  (return false))

(fn `ModifyIntValue`
  (params (ValueName :type Name) (bDelta :type Boolean) (Value :type Integer))
  (returns (ReturnValue :type Boolean))
  (return false))

(fn `ModifyNameValue`
  (params (ValueName :type Name) (NameValue :type Name))
  (returns (ReturnValue :type Boolean))
  (bind _value (`BlueprintMapLibrary.Map_Find` (`/Game/Blueprints/DialogueSystem/W_VNCodex.CodexButtons` (`/Game/Blueprints/DialogueSystem/W_VNMenu.W_Codex` (`self.GameInsMenuWidget`))) NameValue))
  (bind _value_2 (`BlueprintMapLibrary.Map_Find` (`/Game/Blueprints/DialogueSystem/W_VNCodex.CodexButtons` (`/Game/Blueprints/DialogueSystem/W_VNMenu.W_Codex` (`self.GameInsMenuWidget`))) ValueName))
  (switch `name` ValueName
    (:`Default`
      ;[1 1 1] If not doing any of the above, check if triggering flag that updates Codex
      (if (`KismetStringLibrary.StartsWith` (`KismetStringLibrary.Conv_NameToString` ValueName) "CDX_")
        (if (not (`KismetArrayLibrary.Array_Contains` (`self.TriggeredFlags`) NameValue))
          (`KismetArrayLibrary.Array_Add` (`self.TriggeredFlags`) NameValue)
          (`/Game/Blueprints/DialogueSystem/W_CodexButton.UpdateCodexDetails` _value_2)
          (`/Game/Blueprints/DialogueSystem/W_VNDialogue.Notify` (`self.GameInsDialogueWidget`) (`|FormatText` "{CodexName} updated!" (`TextBlock.GetText` (`/Game/Blueprints/DialogueSystem/W_CodexButton.TextBlock_90` _value_2)))))
        (return false)))
    (:`UpdateCodex`
      (`/Game/Blueprints/DialogueSystem/W_CodexButton.UpdateCodexDetails` _value)
      (`/Game/Blueprints/DialogueSystem/W_VNDialogue.Notify` (`self.GameInsDialogueWidget`) (`|FormatText` "{CodexName} updated!" (`TextBlock.GetText` (`/Game/Blueprints/DialogueSystem/W_CodexButton.TextBlock_90` _value)))))
    (:`TriggerFlag`
      ;[1 1 1] Add Flag to Triggered Flags
      (`KismetArrayLibrary.Array_AddUnique` (`self.TriggeredFlags`) NameValue))))

(fn `OnDialogueEvent`
  (params (Context :type "DlgContext Object Reference") (EventName :type Name))
  (returns (ReturnValue :type Boolean))
  (return false))

(fn `PossessNoCamChange`
  (params (PawnToPossess :type "Pawn Object Reference"))
  (returns (ReturnValue :type "Actor Object Reference"))
  (locals (ViewTarget :type "Actor Object Reference"))
  (bind _returnvalue (`GameplayStatics.GetPlayerController` 0))
  (bind _returnvalue_2 (`Controller.GetViewTarget` _returnvalue))
  (bind _output_get (set `local.ViewTarget` _returnvalue_2))
  (`Controller.Possess` _returnvalue PawnToPossess)
  (`PlayerController.SetViewTargetWithBlend` _returnvalue _output_get 0.0 "VTBlend_Linear" 0.0 false)
  (return _returnvalue_2))