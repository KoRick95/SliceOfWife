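; Visual novel helper library whose ToTargetText function turns plain or tagged text into rich text markup.
; It defaults to the Normal style, optionally adds quotes, then parses the text into pieces, tracking the active style tag.
; Pieces matching KeywordStyles, ignoring common punctuation, get that keyword's style before the previous style resumes.
; String replacements optionally switch every tag to its Small variant and close all tags, returning String and Text.
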(fn `ToTargetText`
  (params (InText :type Text) (AddQuotes :type Boolean) (UseSmallStyle :type Boolean))
  (returns (OutString :type String) (OutText :type Text))
  (locals (ProcessedString :type String) (Words :type "Array of String") (KeywordStyles :type "Map of String to String") (CurrentString :type String) (LastTextStyle :type String))
  (bind _currentstring (`local.CurrentString`))
  (bind _processedstring (`local.ProcessedString`))
  (bind (_lefts _rights) (`KismetStringLibrary.Split` (`local.ProcessedString`) ">"))
  (bind _returnvalue (+ (`KismetStringLibrary.FindSubstring` _currentstring ">") 1))
  (bind _returnvalue_2 (`KismetStringLibrary.Replace` (`KismetStringLibrary.Replace` (`KismetStringLibrary.Replace` (`KismetStringLibrary.Replace` (`KismetStringLibrary.Replace` (`KismetStringLibrary.Replace` (`local.CurrentString`) ".") "?") "\"") ",") "!") "'"))
  (bind (_lefts_2 _rights_2) (`KismetStringLibrary.Split` (`local.CurrentString`) _returnvalue_2))
  (bind (_value _returnvalue_3) (`BlueprintMapLibrary.Map_Find` (`local.KeywordStyles`) _returnvalue_2))
  (set `local.ProcessedString` (`KismetTextLibrary.Conv_TextToString` InText))
  (`|ExecutionSequence`
    (:`then_0`
      ;[1 1 1] Make sure text starts with an opening tag
      (if (not (`KismetStringLibrary.StartsWith` (`local.ProcessedString`) "<"))
        (set `local.ProcessedString` (`KismetStringLibrary.Concat_StrStr` "<Normal>" (`local.ProcessedString`)))))
    (:`then_1`
      ;[1 1 1] Add Quotes
      (if AddQuotes
        (set `local.ProcessedString` (`KismetStringLibrary.Concat_StrStr` _lefts ">\"" _rights "\""))))
    (:`then_2`
      (set `local.Words` (`KismetStringLibrary.ParseIntoArray` (`local.ProcessedString`)))
      (set `local.ProcessedString` "")
      (for _array_element (`local.Words`)
        (bind _output_get (set `local.CurrentString` _array_element))
        (if (`KismetStringLibrary.StartsWith` _output_get "<")
          (bind _output_get_2 (set `local.LastTextStyle` (`KismetStringLibrary.GetSubstring` _currentstring 0 _returnvalue)))
          (set `local.ProcessedString` (`KismetStringLibrary.Concat_StrStr` (`local.ProcessedString`) _output_get_2))
          (set `local.CurrentString` (`KismetStringLibrary.RightChop` (`local.CurrentString`) _returnvalue)))
        (if _returnvalue_3
          (set `local.ProcessedString` (`KismetStringLibrary.Concat_StrStr` (`local.ProcessedString`) _lefts_2 _value _returnvalue_2 (`local.LastTextStyle`) _rights_2 " "))
          (else
            (set `local.ProcessedString` (`KismetStringLibrary.Concat_StrStr` (`local.ProcessedString`) (`local.CurrentString`) " "))))))
    (:`then_3`
      (if UseSmallStyle
        (`KismetStringLibrary.ReplaceInline` (`local.ProcessedString`) ">" "Small>")))
    (:`then_4`
      ;[1 1 1] Close all tags
      (`KismetStringLibrary.ReplaceInline` (`local.ProcessedString`) "<" "</><")
      (set `local.ProcessedString` (`KismetStringLibrary.RightChop` (`local.ProcessedString`) 3)))
    (:`then_5`
      ;[1 1 1] Close last style tag
      (set `local.ProcessedString` (`KismetStringLibrary.Concat_StrStr` (`local.ProcessedString`) "</>")))
    (:`then_6`
      (return _processedstring (`KismetTextLibrary.Conv_StringToText` _processedstring)))))