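; Blueprint function library for the dialogue system, with a rich-text formatter and a float interpolation helper.
; ToTargetText ensures an opening style tag, optionally adds quotes, then wraps words found in KeywordStyles, ignoring punctuation, in their keyword style.
; It restores the preceding style after each keyword and inserts closing tags throughout.
; FakeLerp steps a float toward a target at constant speed, clamping to avoid overshoot.
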(fn `FakeLerp`
  (params (CurrentValue :type "Float (double-precision)") (TargetValue :type "Float (double-precision)") (DeltaTime :type "Float (double-precision)") (Speed :type "Float (double-precision)"))
  (returns (Output :type "Float (double-precision)"))
  (bind _returnvalue (< CurrentValue TargetValue))
  (bind _returnvalue_2 (+ (* DeltaTime Speed (`KismetMathLibrary.SelectFloat` 1.0 -1.0 _returnvalue)) CurrentValue))
  (return (`KismetMathLibrary.SelectFloat` (`KismetMathLibrary.FMin` _returnvalue_2 TargetValue) (`KismetMathLibrary.FMax` _returnvalue_2 TargetValue) _returnvalue)))

(fn `ToTargetText`
  (params (InText :type Text) (AddQuotes :type Boolean))
  (returns (OutString :type String) (OutText :type Text))
  (locals (ProcessedString :type String) (Words :type "Array of String") (KeywordStyles :type "Map of String to String") (CurrentString :type String) (LastTextStyle :type String))
  (bind _currentstring (`local.CurrentString`))
  (bind _processedstring (`local.ProcessedString`))
  (bind (_lefts _rights) (`KismetStringLibrary.Split` (`local.ProcessedString`) ">"))
  (bind _returnvalue (+ (`KismetStringLibrary.FindSubstring` _currentstring ">") 1))
  (bind _returnvalue_2 (`KismetStringLibrary.Replace` (`KismetStringLibrary.Replace` (`KismetStringLibrary.Replace` (`KismetStringLibrary.Replace` (`KismetStringLibrary.Replace` (`KismetStringLibrary.Replace` (`local.CurrentString`) ".") "?") "\"") ",") "!") "'"))
  (bind (_lefts_2 _rights_2) (`KismetStringLibrary.Split` (`local.CurrentString`) _returnvalue_2))
  (bind (_value _returnvalue_3) (`BlueprintMapLibrary.Map_Find` (`local.KeywordStyles`) _returnvalue_2))
  (set `local.ProcessedString` (`KismetTextLibrary.Conv_TextToString` InText))
  (`|ExecutionSequence`
    (:`then_0`
      ;[1 1 1] Make sure text starts with an opening tag
      (if (not (`KismetStringLibrary.StartsWith` (`local.ProcessedString`) "<"))
        (set `local.ProcessedString` (`KismetStringLibrary.Concat_StrStr` "<Normal>" (`local.ProcessedString`)))))
    (:`then_1`
      ;[1 1 1] Add Quotes
      (if AddQuotes
        (set `local.ProcessedString` (`KismetStringLibrary.Concat_StrStr` _lefts ">\"" _rights "\""))))
    (:`then_2`
      (set `local.Words` (`KismetStringLibrary.ParseIntoArray` (`local.ProcessedString`)))
      (set `local.ProcessedString` "")
      (for _array_element (`local.Words`)
        (bind _output_get (set `local.CurrentString` _array_element))
        (if (`KismetStringLibrary.StartsWith` _output_get "<")
          (bind _output_get_2 (set `local.LastTextStyle` (`KismetStringLibrary.GetSubstring` _currentstring 0 _returnvalue)))
          (set `local.ProcessedString` (`KismetStringLibrary.Concat_StrStr` (`local.ProcessedString`) _output_get_2))
          (set `local.CurrentString` (`KismetStringLibrary.RightChop` (`local.CurrentString`) _returnvalue)))
        (if _returnvalue_3
          (set `local.ProcessedString` (`KismetStringLibrary.Concat_StrStr` (`local.ProcessedString`) _lefts_2 _value _returnvalue_2 (`local.LastTextStyle`) _rights_2 " "))
          (else
            (set `local.ProcessedString` (`KismetStringLibrary.Concat_StrStr` (`local.ProcessedString`) (`local.CurrentString`) " "))))))
    (:`then_3`
      ;[1 1 1] Close all tags
      (`KismetStringLibrary.ReplaceInline` (`local.ProcessedString`) "<" "</><")
      (set `local.ProcessedString` (`KismetStringLibrary.RightChop` (`local.ProcessedString`) 3)))
    (:`then_4`
      ;[1 1 1] Close last style tag
      (set `local.ProcessedString` (`KismetStringLibrary.Concat_StrStr` (`local.ProcessedString`) "</>")))
    (:`then_5`
      (return _processedstring (`KismetTextLibrary.Conv_StringToText` _processedstring)))))