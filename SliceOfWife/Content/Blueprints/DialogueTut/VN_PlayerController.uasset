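; Player controller for a visual novel dialogue game that toggles between the dialogue screen and the menu.
; On release of the Toggle Game/Menu input, it gets the menu widget from the VN game instance and acts only while in game.
; The canvas panel's visibility decides the switch: when hit-test invisible it shows the menu, otherwise it returns to the dialogue widget.
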(event `InputAction|Toggle Game/Menu`
  (params (Key :type "Key Structure"))
  (bind _menuwidget (`/Game/Blueprints/DialogueTut/VN_GameInstance.MenuWidget` (cast `/Game/Blueprints/DialogueTut/VN_GameInstance` (`GameplayStatics.GetGameInstance`) :!pure true)))
  (:`Released`
    (if (`/Game/Blueprints/DialogueTut/W_VNMenu.IsInGame` _menuwidget)
      (if (`|EnumEquality` (`Widget.GetVisibility` (`/Game/Blueprints/DialogueTut/W_VNMenu.CanvasPanel_0` _menuwidget)) "HitTestInvisible")
        (`/Game/Blueprints/DialogueTut/W_VNMenu.ShowMenuWidget` _menuwidget 1)
        (else
          (`/Game/Blueprints/DialogueTut/W_VNMenu.ShowDialogueWidget` _menuwidget))))))

(fn `UserConstructionScript`)