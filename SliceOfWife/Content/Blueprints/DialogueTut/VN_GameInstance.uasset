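; Game instance for a visual novel that owns persistent save data, the UI widgets and triggered story flags.
; Init loads or creates the VN_PersistantData save, then builds and cross-links menu, dialogue, options, codex and gallery widgets; Shutdown saves it.
; It also acts as a dialogue participant, testing flags as conditions and using name-value changes to set flags or update codex entries with notifications.
; New game clears flags and resets player name, history, dialogue and codex.
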(event `self.ReceiveInit`
  (bind _w_options (`/Game/Blueprints/DialogueTut/W_Menu.W_Options` (`self.MenuWidget`)))
  (bind _w_codex (`/Game/Blueprints/DialogueTut/W_Menu.W_Codex` (`self.MenuWidget`)))
  (`/Engine/EditorBlueprintResources/StandardMacros.IsValid` (`self.PersistantData`)
    (:`Is Not Valid`
      (`|ExecutionSequence`
        (:`then_0`
          ;[1 1 1] Get Persistant Data
          (bind _returnvalue (`GameplayStatics.DoesSaveGameExist` "VN_PersistantData"))
          (if _returnvalue
            (bind _returnvalue_2 (`GameplayStatics.LoadGameFromSlot` "VN_PersistantData"))
            (set `self.PersistantData` (cast `/Game/Blueprints/DialogueTut/VN_PersistantData` _returnvalue_2 :!pure true))
            (else
              (bind _returnvalue_3 (`GameplayStatics.CreateSaveGameObject` "/Game/Blueprints/DialogueTut/VN_PersistantData.VN_PersistantData_C"))
              (bind _output_get (set `self.PersistantData` _returnvalue_3))
              (set `/Game/Blueprints/DialogueTut/VN_PersistantData.ShowUnselectableOptions` false _output_get)
              (set `/Game/Blueprints/DialogueTut/VN_PersistantData.TextSpeed` 0.001 _output_get))))
        (:`then_1`
          ;[1 1 1] Create Widgets and Initialise Options
          (bind _returnvalue_4 (`|CreateWidget` "/Game/Blueprints/DialogueTut/W_Menu.W_Menu_C"))
          (bind _output_get_2 (set `self.MenuWidget` _returnvalue_4))
          (bind _returnvalue_5 (`|CreateWidget` "/Game/Blueprints/UI/W_Dialogue.W_Dialogue_C" null _output_get_2 (`/Game/Blueprints/DialogueTut/W_Menu.W_History` _output_get_2) (`self.PersistantData`)))
          (bind _output_get_3 (set `/Game/Blueprints/DialogueTut/W_Menu.DialogueWidget` _returnvalue_5 _output_get_2))
          (set `self.DialogueWidget` _output_get_3)
          (bind _output_get_4 (set `self.OptionsWidget` _w_options))
          (set `/Game/Blueprints/DialogueTut/W_Options.DialogueWidget` (`self.DialogueWidget`) _output_get_4)
          (set `/Game/Blueprints/DialogueTut/W_Options.VNPersistantData` (`self.PersistantData`) _w_options)
          (`/Game/Blueprints/DialogueTut/W_Options.InitialiseSavedOptions` _w_options)
          (bind _output_get_5 (set `self.CodexWidget` _w_codex))
          (`/Game/Blueprints/DialogueTut/W_Codex.CreateCodexButtons` _w_codex (`self.DialogueWidget`))
          (`/Game/Blueprints/DialogueTut/W_Codex.CreateCodexButtons` _output_get_5 (`self.DialogueWidget`))
          (bind _returnvalue_6 (`|CreateWidget` "/Game/Blueprints/DialogueTut/W_GalleryImage.W_GalleryImage_C" null (`self.PersistantData`)))
          (`/Game/Blueprints/DialogueTut/W_Gallery.CreateGalleryButtons` (`/Game/Blueprints/DialogueTut/W_Menu.W_Gallery` (`self.MenuWidget`)) (`self.PersistantData`) _returnvalue_6))))))

(event `self.ReceiveShutdown`
  ;[1 1 1] Save Persistant Data on Shutdown
  (`GameplayStatics.SaveGameToSlot` (`self.PersistantData`) "VN_PersistantData"))

(event `/Game/Blueprints/DialogueTut/VN_SaveInterface.OnNewGame`
  (bind _buttonscrollbox (`/Game/Blueprints/DialogueTut/W_Codex.ButtonScrollBox` (`self.CodexWidget`)))
  (`KismetArrayLibrary.Array_Clear` (`self.TriggeredFlags`))
  (set `self.PlayerName` "???")
  (`/Game/Blueprints/DialogueTut/W_History.OnNewGame` (`/Game/Blueprints/DialogueTut/W_Menu.W_History` (`self.MenuWidget`)))
  (`/Game/Blueprints/DialogueTut/W_History.OnNewGame` (`self.DialogueWidget`))
  (for _index (range (`PanelWidget.GetChildrenCount` _buttonscrollbox))
    (`/Game/Blueprints/DialogueTut/W_CodexButton.UpdateCodexDetails` (cast `/Game/Blueprints/DialogueTut/W_CodexButton` (`PanelWidget.GetChildAt` _buttonscrollbox _index) :!pure true))))

(fn `CheckCondition`
  (params (Context :type "DlgContext Object Reference") (ConditionName :type Name))
  (returns (ReturnValue :type Boolean))
  (return (`KismetArrayLibrary.Array_Contains` (`self.TriggeredFlags`) ConditionName)))

(fn `GetBoolValue`
  (params (ValueName :type Name))
  (returns (ReturnValue :type Boolean))
  (return false))

(fn `GetFloatValue`
  (params (ValueName :type Name))
  (returns (ReturnValue :type "Float (double-precision)"))
  (return 0.0))

(fn `GetIntValue`
  (params (ValueName :type Name))
  (returns (ReturnValue :type Integer))
  (return 0))

(fn `GetNameValue`
  (params (ValueName :type Name))
  (returns (ReturnValue :type Name))
  (return "None"))

(fn `GetParticipantDisplayName`
  (params (ActiveSpeaker :type Name))
  (returns (ReturnValue :type Text))
  (return ""))

(fn `GetParticipantGender`
  (returns (ReturnValue :type "ETextGender Enum"))
  (return "Masculine"))

(fn `GetParticipantIcon`
  (params (ActiveSpeaker :type Name) (ActiveSpeakerState :type Name))
  (returns (ReturnValue :type "Texture2D Object Reference"))
  (return null))

(fn `GetParticipantName`
  (returns (ReturnValue :type Name))
  (return "VNGameInstance"))

(fn `ModifyBoolValue`
  (params (ValueName :type Name) (bNewValue :type Boolean))
  (returns (ReturnValue :type Boolean))
  (return false))

(fn `ModifyFloatValue`
  (params (ValueName :type Name) (bDelta :type Boolean) (Value :type "Float (double-precision)"))
  (returns (ReturnValue :type Boolean))
  (return false))

(fn `ModifyIntValue`
  (params (ValueName :type Name) (bDelta :type Boolean) (Value :type Integer))
  (returns (ReturnValue :type Boolean))
  (return false))

(fn `ModifyNameValue`
  (params (ValueName :type Name) (NameValue :type Name))
  (returns (ReturnValue :type Boolean))
  (bind _value (`BlueprintMapLibrary.Map_Find` (`/Game/Blueprints/DialogueTut/W_Codex.CodexButtons` (`/Game/Blueprints/DialogueTut/W_Menu.W_Codex` (`self.MenuWidget`))) NameValue))
  (bind _value_2 (`BlueprintMapLibrary.Map_Find` (`/Game/Blueprints/DialogueTut/W_Codex.CodexButtons` (`/Game/Blueprints/DialogueTut/W_Menu.W_Codex` (`self.MenuWidget`))) ValueName))
  (switch `name` ValueName
    (:`Default`
      ;[1 1 1] If not doing any of the above, check if triggering flag that updates Codex
      (if (`KismetStringLibrary.StartsWith` (`KismetStringLibrary.Conv_NameToString` ValueName) "CDX_")
        (if (not (`KismetArrayLibrary.Array_Contains` (`self.TriggeredFlags`) NameValue))
          (`KismetArrayLibrary.Array_Add` (`self.TriggeredFlags`) NameValue)
          (`/Game/Blueprints/DialogueTut/W_CodexButton.UpdateCodexDetails` _value_2)
          (`/Game/Blueprints/UI/W_Dialogue.Notify` (`self.DialogueWidget`) (`|FormatText` "{CodexName} updated!" (`TextBlock.GetText` (`/Game/Blueprints/DialogueTut/W_CodexButton.TextBlock_90` _value_2)))))
        (return false)))
    (:`UpdateCodex`
      (`/Game/Blueprints/DialogueTut/W_CodexButton.UpdateCodexDetails` _value)
      (`/Game/Blueprints/UI/W_Dialogue.Notify` (`self.DialogueWidget`) (`|FormatText` "{CodexName} updated!" (`TextBlock.GetText` (`/Game/Blueprints/DialogueTut/W_CodexButton.TextBlock_90` _value)))))
    (:`TriggerFlag`
      ;[1 1 1] Add Flag to Triggered Flags
      (`KismetArrayLibrary.Array_AddUnique` (`self.TriggeredFlags`) NameValue))))

(fn `OnDialogueEvent`
  (params (Context :type "DlgContext Object Reference") (EventName :type Name))
  (returns (ReturnValue :type Boolean))
  (return false))