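; Visual novel game mode that sets up the menu and dialogue UI when play begins.
; It reads both widgets from VN_GameInstance and branches on the menu's IsInGame check.
; If in game, it makes the menu's root canvas transparent and hit-test invisible.
; Otherwise it adds the dialogue widget to the viewport, followed by the menu widget.
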(event `self.ReceiveBeginPlay`
  (bind _asvn_game_instance (cast `/Game/Blueprints/DialogueTut/VN_GameInstance` (`GameplayStatics.GetGameInstance`) :!pure true))
  (bind _menuwidget (`/Game/Blueprints/DialogueTut/VN_GameInstance.MenuWidget` _asvn_game_instance))
  (bind _canvaspanel_0 (`/Game/Blueprints/DialogueTut/W_VNMenu.CanvasPanel_0` _menuwidget))
  (if (`/Game/Blueprints/DialogueTut/W_VNMenu.IsInGame` _menuwidget)
    (`Widget.SetRenderOpacity` _canvaspanel_0 0.0)
    (`Widget.SetVisibility` _canvaspanel_0 "HitTestInvisible")
    (else
      (`UserWidget.AddToViewport` (`/Game/Blueprints/DialogueTut/VN_GameInstance.DialogueWidget` _asvn_game_instance) 0)
      (`UserWidget.AddToViewport` _menuwidget 0))))

(fn `UserConstructionScript`)