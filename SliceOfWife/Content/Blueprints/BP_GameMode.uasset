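; Game mode Blueprint that sets up the menu and dialogue UI when play begins.
; It uses the MenuWidget held by BP_GameInstance and branches on its IsInGame check.
; When in game, the menu's canvas panel becomes fully transparent and HitTestInvisible.
; Otherwise, the nested DialogueWidget is added to the viewport, followed by the menu itself.
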(event `self.ReceiveBeginPlay`
  (bind _menuwidget (`/Game/Blueprints/BP_GameInstance.MenuWidget` (cast `/Game/Blueprints/BP_GameInstance` (`GameplayStatics.GetGameInstance`) :!pure true)))
  (bind _canvaspanel_0 (`/Game/Blueprints/UI/W_Menu.CanvasPanel_0` _menuwidget))
  (if (`/Game/Blueprints/UI/W_Menu.IsInGame` _menuwidget)
    (`Widget.SetRenderOpacity` _canvaspanel_0 0.0)
    (`Widget.SetVisibility` _canvaspanel_0 "HitTestInvisible")
    (else
      (`UserWidget.AddToViewport` (`/Game/Blueprints/UI/W_Menu.DialogueWidget` _menuwidget) 0)
      (`UserWidget.AddToViewport` _menuwidget 0))))

(fn `UserConstructionScript`)