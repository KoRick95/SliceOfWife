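; Player character Blueprint that adds the player HUD at startup and lets the player interact with reception objects.
; A box collider stores an overlapped BP_Reception as the current interactable and toggles its focus, and the Interact input calls it when usable.
; Mouse up/down pitches the camera component locally, while horizontal look is unwired.
; Camera manager view pitch is limited to a narrow range on BeginPlay.
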(event `self.ReceiveBeginPlay`
  (`self.Set Cam Min Max`)
  (set `self.Collider_Var` (`self.CapsuleComponent`))
  (bind _returnvalue (`|CreateWidget` "/Game/Blueprints/UI/W_PlayerHUD.W_PlayerHUD_C" null self))
  (`UserWidget.AddToViewport` _returnvalue 0))

(event `self.BoxCollider.OnComponentBeginOverlap`
  (params (OverlappedComponent :type "PrimitiveComponent Object Reference") (OtherActor :type "Actor Object Reference") (OtherComp :type "PrimitiveComponent Object Reference") (OtherBodyIndex :type Integer) (bFromSweep :type Boolean) (SweepResult :type "HitResult Structure (by ref)"))
  (if (`KismetMathLibrary.ClassIsChildOf` (`GameplayStatics.GetObjectClass` OtherActor) "/Game/Blueprints/InteractableEnvironment/BP_Reception.BP_Reception_C")
    (bind _asbp_reception (cast `/Game/Blueprints/InteractableEnvironment/BP_Reception` OtherActor))
    (set `self.CurrentInteractable` (make `/Game/Blueprints/Structures/ST_Interactable` _asbp_reception true))
    (bind _interactenabled (`/Game/Blueprints/InteractableEnvironment/BP_Reception.RefreshInteraction` _asbp_reception))
    (if _interactenabled
      (`/Game/Blueprints/InteractableEnvironment/BP_Reception.IsFocused` _asbp_reception))))

(event `self.BoxCollider.OnComponentEndOverlap`
  (params (OverlappedComponent :type "PrimitiveComponent Object Reference") (OtherActor :type "Actor Object Reference") (OtherComp :type "PrimitiveComponent Object Reference") (OtherBodyIndex :type Integer))
  (bind _currentinteractable_reception (break `/Game/Blueprints/Structures/ST_Interactable` (`self.CurrentInteractable`)))
  (if (== OtherActor _currentinteractable_reception)
    (`/Game/Blueprints/InteractableEnvironment/BP_Reception.IsUnfocused` _currentinteractable_reception)
    (set `self.CurrentInteractable` (make `/Game/Blueprints/Structures/ST_Interactable` null))))

(event `InputAction|Interact`
  (params (Key :type "Key Structure"))
  (bind (_currentinteractable_reception _currentinteractable_canuse) (break `/Game/Blueprints/Structures/ST_Interactable` (`self.CurrentInteractable`)))
  (:`Pressed`
    (`self.Interact`)
    (if _currentinteractable_canuse
      (`/Game/Blueprints/InteractableEnvironment/BP_Reception.Interact` _currentinteractable_reception))))

(event `InputAxis|MouseLookRight`
  (params (AxisValue :type "Float (single-precision)")))

(event `InputAxis|MouseLookUp`
  (params (AxisValue :type "Float (single-precision)"))
  (`SceneComponent.K2_AddLocalRotation` (`self.Camera`) (`KismetMathLibrary.MakeRotator` 0.0 AxisValue) false false))

(fn `Set Cam Min Max`
  (bind _returnvalue (`GameplayStatics.GetPlayerCameraManager` 0))
  (set `PlayerCameraManager.ViewPitchMin` -10.0 _returnvalue)
  (set `PlayerCameraManager.ViewPitchMax` 10.0 _returnvalue))

(fn `UserConstructionScript`)