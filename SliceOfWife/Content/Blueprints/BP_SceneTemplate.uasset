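; BP_SceneTemplate is a dialogue scene actor that plays lines from a data table, one at a time.
; InitiateNewScene loads the table's rows into an array and shows a W_DisplayDialogue widget with each line's text and speaker name.
; The Interact input advances lines, gated by a one-second delay after each appears.
; After the last row, it removes the widget, clears ScenePlaying on SceneStartActor and destroys itself.
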(event `self.ReceiveBeginPlay`
  (`self.EnableInput` (`GameplayStatics.GetPlayerController` 0)))

(event `InitiateNewScene`
  (params (CurrentScene :type "DataTable Object Reference"))
  (bind _outrownames (`DataTableFunctionLibrary.GetDataTableRowNames` CurrentScene))
  (for _array_element _outrownames
    (bind _returnvalue (`|GetDataTableRow` CurrentScene _array_element)
      (:`then`
        (`KismetArrayLibrary.Array_Add` (`self.ArrayOfRows`) _returnvalue))))
  (bind _returnvalue_2 (`|CreateWidget` "/Game/UI/W_DisplayDialogue.W_DisplayDialogue_C"))
  (bind _output_get (set `self.DisplayDialogueWidget` _returnvalue_2))
  (`UserWidget.AddToViewport` _output_get 0)
  (`self.PlayLine`))

(event `PlayLine`
  (bind _displaydialoguewidget (`self.DisplayDialogueWidget`))
  (bind (_speaker _text) (break `/Game/Assets/Structs/VN_SceneStruct` (`|GetArrayItem` (`self.ArrayOfRows`) (`self.Row`))))
  (set `self.RowFinished` false)
  (if (>= (`self.Row`) (`KismetArrayLibrary.Array_Length` (`self.ArrayOfRows`)))
    (`self.EndScene`)
    (else
      (`/Engine/EditorBlueprintResources/StandardMacros.IsValid` _displaydialoguewidget
        (:`Is Valid`
          (set `/Game/UI/W_DisplayDialogue.Text` (`KismetTextLibrary.Conv_StringToText` _text) _displaydialoguewidget)
          (`TextBlock.SetText` (`/Game/UI/W_DisplayDialogue.SpeakerName` _displaydialoguewidget) (`KismetTextLibrary.Conv_StringToText` (`|GetEnumeratorNameAsString` _speaker)))
          (`KismetSystemLibrary.Delay` 1.0)
          (set `self.RowFinished` true))))))

(event `InputAction|Interact`
  (params (Key :type "Key Structure"))
  (:`Pressed`
    (if (`self.RowFinished`)
      (set `self.Row` (+ (`self.Row`) 1))
      (`self.PlayLine`))))

(event `EndScene`
  (`Widget.RemoveFromParent` (`self.DisplayDialogueWidget`))
  (set `/Game/Blueprints/BP_NPCTouchClick.ScenePlaying` false (`self.SceneStartActor`))
  (`self.K2_DestroyActor`))

(fn `UserConstructionScript`)